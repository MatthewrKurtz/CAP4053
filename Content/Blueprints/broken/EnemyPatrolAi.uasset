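; Enemy AI controller with two behaviours: a Charger that repeatedly chases the player and a Patrol that moves between points.
; BeginPlay switches on an unconnected empty string to start a timer for either behaviour, so neither named case matches as written.
; TrackPlayer uses AI MoveTo, while MoveToPatrolPoint moves straight to the pawn's current patrol point without pathfinding.
; The patrol step calls GetRandomLocation on the pawn and flags it moving after a short delay.
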(event Custom|TrackPlayer
  (AI|AIMoveTo (Pawn|GetControlledPawn) "0, 0, 0" (Game|GetPlayerCharacter 0) 5.0 false))

(event Custom|MoveToPatrolPoint
  (Utilities|FlowControl|Sequence
    (:then_0
      (bind _asenemy_character_patrol (Utilities|Casting|CastToEnemyCharacter_Patrol (Pawn|GetControlledPawn)))
      (AI|Navigation|MovetoLocation (Utilities|Array|Get(acopy) (Variables|/Game/Blueprints/broken/EnemyCharacter_Patrol.EnemyCharacter_Patrol_C|GetPatrolPoints _asenemy_character_patrol) (Variables|/Game/Blueprints/broken/EnemyCharacter_Patrol.EnemyCharacter_Patrol_C|GetCurrentPatrolPoint _asenemy_character_patrol)) -1.0 true false false true 0)
      (Utilities|FlowControl|Delay 0.2)
      (bind _output_get (Variables|/Game/Blueprints/broken/EnemyCharacter_Patrol.EnemyCharacter_Patrol_C|SetisMoving _asenemy_character_patrol true))
      (Development|PrintString (Utilities|String|ToString(Boolean) _output_get)))
    (:then_1
      (Default|GetRandomLocation _asenemy_character_patrol))))

(event EventBeginPlay
  (switch string ""
    (:Charger
      (Utilities|Time|SetTimerbyFunctionName 0 "TrackPlayer" 5.0 true))
    (:Patrol
      (Utilities|Time|SetTimerbyFunctionName 0 "MoveToPatrolPoint" 5.0))))

(event EventTick
  (params (DeltaSeconds :type Float%20%28single-precision%29)))

(fn ConstructionScript)