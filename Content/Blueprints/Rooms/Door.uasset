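; Door actor Blueprint for rooms that removes nearby doors when it is destroyed.
; On Destroyed, it scans all Door actors for ones nearer than Closest and farther than Min.
; Each new nearest match updates Closest and is destroyed immediately inside the loop, so several doors can go.
; A distance-threshold check before destruction is disconnected, and the construction script is empty.
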(event EventDestroyed
  (bind _outactors (Actor|GetAllActorsOfClass "Door_C"))
  (for _array_element _outactors
    (if (and (< (Transformation|GetDistanceTo _array_element) (Variables|Default|GetClosest)) (> (Transformation|GetDistanceTo _array_element) (Variables|Default|Getmin)))
      (bind _output_get (Variables|Default|SetClosestActor _array_element))
      (bind _output_get_2 (Variables|Default|SetClosest (Transformation|GetDistanceTo _array_element)))
      (Actor|DestroyActor _output_get))))

(fn ConstructionScript)