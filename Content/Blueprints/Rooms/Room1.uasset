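; Room actor for a twin-stick game that spawns four doors at its box components and an enemy spawner above its root on BeginPlay.
; Overlap by a "Friendly" actor moves the game mode's camera above the room.
; The spawner receives a room reference and raises Count, which DecrementCount lowers.
; Tick's zero-count DoOnce leads nowhere, as the door-destruction and neighbor-detection logic is disconnected.
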(event Custom|Decrement%20Count
  ;[1 1 1] Decrement count when enemies die
  (bind _result (Math|Integer|DecrementInt (Variables|Default|GetCount))
    (:%20%20
      (Variables|Default|SetCount _result))))

(event EventBeginPlay
  (bind _box1 (Variables|Default|GetBox1))
  (bind _box3 (Variables|Default|GetBox3))
  (bind _box2 (Variables|Default|GetBox2))
  (bind _defaultsceneroot (Variables|Default|GetDefaultSceneRoot))
  (bind _box (Variables|Default|GetBox))
  (bind _returnvalue (Transformation|GetWorldTransform _box2))
  (bind _returnvalue_2 (Transformation|GetWorldTransform _box3))
  (bind _returnvalue_3 (Transformation|GetWorldTransform _box))
  (bind _returnvalue_4 (Transformation|GetWorldTransform _box1))
  (bind _returnvalue_5 (Transformation|GetWorldTransform _defaultsceneroot))
  ;[1 1 1] Spawn doors
  (bind _returnvalue_6 (Game|SpawnActorfromClass "/Game/Blueprints/Rooms/Door.Door_C" (Math|Transform|MakeTransform (Math|Vector|MakeVector (.x (.location _returnvalue_3)) (.y (.location _returnvalue_3)) (.z (.location _returnvalue_3))) "0, 0, 0" "1,1,1") "Undefined" 0 0))
  (Variables|Default|SetEast _returnvalue_6)
  (bind _returnvalue_7 (Game|SpawnActorfromClass "/Game/Blueprints/Rooms/Door.Door_C" (Math|Transform|MakeTransform (Math|Vector|MakeVector (.x (.location _returnvalue_2)) (.y (.location _returnvalue_2)) (.z (.location _returnvalue_2))) "0, 0, 0" "1,1,1") "Undefined" 0 0))
  (Variables|Default|SetWest _returnvalue_7)
  (bind _returnvalue_8 (Game|SpawnActorfromClass "/Game/Blueprints/Rooms/Door.Door_C" (Math|Transform|MakeTransform (Math|Vector|MakeVector (.x (.location _returnvalue_4)) (.y (.location _returnvalue_4)) (.z (.location _returnvalue_4))) (Math|Rotator|MakeRotator (.roll (.rotation _returnvalue_4)) (.pitch (.rotation _returnvalue_4)) (+ (.yaw (.rotation _returnvalue_4)) (Math|Conversions|ToFloat(Integer) (Variables|Default|GetRotate)))) "1,1,1") "Undefined" 0 0))
  (Variables|Default|SetSouth _returnvalue_8)
  (bind _returnvalue_9 (Game|SpawnActorfromClass "/Game/Blueprints/Rooms/Door.Door_C" (Math|Transform|MakeTransform (Math|Vector|MakeVector (.x (.location _returnvalue)) (.y (.location _returnvalue)) (.z (.location _returnvalue))) (Math|Rotator|MakeRotator (.roll (.rotation _returnvalue)) (.pitch (.rotation _returnvalue)) (+ (.yaw (.rotation _returnvalue)) (Math|Conversions|ToFloat(Integer) (Variables|Default|GetRotate)))) "1,1,1") "Undefined" 0 0))
  (Variables|Default|SetNorth _returnvalue_9)
  ;[1 1 1] Spawn one enemy, and add to the count
  (bind _returnvalue_10 (Game|SpawnActorfromClass "/Game/Blueprints/Enemies/EnemySpawner.EnemySpawner_C" (Math|Transform|MakeTransform (Math|Vector|MakeVector (.x (.location _returnvalue_5)) (.y (.location _returnvalue_5)) (+ (.z (.location _returnvalue_5)) (Math|Conversions|ToFloat(Integer) 150))) (.rotation _returnvalue_5) (.scale _returnvalue_5)) "Undefined" 0 0))
  (bind _result (Math|Integer|IncrementInt (Variables|Default|GetCount))
    (:%20%20
      (Variables|Default|SetCount _result)
      (Variables|/Game/Blueprints/Enemies/EnemySpawner.EnemySpawner_C|SetcurrentRoom _returnvalue_10 self))))

(event Collision|EventActorBeginOverlap
  (params (OtherActor :type Actor%20Object%20Reference))
  (bind _defaultsceneroot (Variables|Default|GetDefaultSceneRoot))
  (bind _returnvalue (Transformation|GetWorldLocation _defaultsceneroot))
  ;[1 1 1] Camera switch to appropriate room
  (if (Actor|ActorHasTag OtherActor "Friendly")
    (bind _astwin_stick_mode (Utilities|Casting|CastToTwinStickMode (Game|GetGameMode)))
    (Transformation|SetWorldLocation (Variables|/Script/Engine.Actor|GetRootComponent (Variables|/Game/Blueprints/TwinStickMode.TwinStickMode_C|GetCameraReference _astwin_stick_mode)) (Math|Vector|MakeVector (.x _returnvalue) (.y _returnvalue) (+ (.z _returnvalue) 1.75e+03)) false false)))

(event EventTick
  (params (DeltaSeconds :type Float%20%28single-precision%29))
  ;[1 1 1] To destroy appropriate doors
  (if (== (Variables|Default|GetCount) 0)
    (Utilities|FlowControl|DoOnce false)))

(fn ConstructionScript)