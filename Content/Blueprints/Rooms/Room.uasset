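; Room actor for a twin-stick game that handles its doors, layout, enemies and camera position.
; BeginPlay builds a tile grid from floor bounds, spawns four doors and populates the spawn room.
; Friendly overlap moves the camera and, on first entry, spawns obstacles and enemies from DT_RoomLayouts.
; Tick destroys the doors selected by RoomInfo once an entered room's enemy count reaches zero.
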(event Custom|RemoveEnemy
  (params (EnemyToBeRemoved :type Enemy%20Character%20Object%20Reference))
  ;[1 1 1] Decrement count when enemies die
  (Utilities|Array|RemoveItem (Variables|Default|GetEnemiesInTheRoom) EnemyToBeRemoved)
  (Math|Integer|DecrementInt (Variables|Default|GetCurrentEnemyCount)))

(event Custom|CreateGridUnits
  ;[1 1 1] Find the location of the topright and bottom left corners that the grid needs to be
  (bind _returnvalue (Game|SpawnActorfromClass "/Game/Blueprints/Rooms/TestUnit.TestUnit_C" (Math|Transform|MakeTransform (Variables|Default|GetTopRightCornerOfFloor) "0, 0, 0" "1,1,1") "Undefined" 0 0))
  (Variables|Default|SetTopRightGridLocation (CallFunction|GetTopRightCornerOfRoom _returnvalue))
  (Transformation|SetActorLocation _returnvalue (CallFunction|GetTopRightCornerOfRoom _returnvalue) false true)
  (bind _returnvalue_2 (Game|SpawnActorfromClass "/Game/Blueprints/Rooms/TestUnit.TestUnit_C" (Math|Transform|MakeTransform (Variables|Default|GetTopRightCornerOfFloor) "0, 0, 0" "1,1,1") "Undefined" 0 0))
  (Variables|Default|SetBottomLeftGridLocation (CallFunction|GetBottomLeftCornerOfRoom _returnvalue_2))
  (Transformation|SetActorLocation _returnvalue_2 (CallFunction|GetBottomLeftCornerOfRoom _returnvalue_2) false true)
  (Actor|DestroyActor _returnvalue_2)
  (Actor|DestroyActor _returnvalue)
  ;[1 1 1] Spawn the appropriate number of grid units inside the room
  (for _index (range 0 (- (Variables|Default|GetNumberOfGridTiles_Y) 1))
    (bind _returnvalue_3 (Utilities|Array|Add (Variables|Default|GetGrid) (Utilities|Struct|MakeFGridCols (Utilities|Array|MakeArray "0, 0, 0"))))
    (for _index_2 (range 0 (- (Variables|Default|GetNumberOfGridTiles_X) 1))
      (if (== _index_2 0)
        (Utilities|Array|RemoveIndex (Utilities|Struct|BreakFGridCols (Utilities|Array|Get(acopy) (Variables|Default|GetGrid) _returnvalue_3)))
        (Utilities|Array|Add (Utilities|Struct|BreakFGridCols (Utilities|Array|Get(acopy) (Variables|Default|GetGrid) _returnvalue_3)) (- (Variables|Default|GetTopRightGridLocation) (Math|Vector|MakeVector (* _index_2 (/ (.x (- (Variables|Default|GetTopRightGridLocation) (Variables|Default|GetBottomLeftGridLocation))) (Math|Conversions|ToFloat(Integer) (- (Variables|Default|GetNumberOfGridTiles_X) 1)))) (* _index (/ (.y (- (Variables|Default|GetTopRightGridLocation) (Variables|Default|GetBottomLeftGridLocation))) (Math|Conversions|ToFloat(Integer) (- (Variables|Default|GetNumberOfGridTiles_Y) 1)))) 0.0)))
        (else
          (Utilities|Array|Add (Utilities|Struct|BreakFGridCols (Utilities|Array|Get(acopy) (Variables|Default|GetGrid) _returnvalue_3)) (- (Variables|Default|GetTopRightGridLocation) (Math|Vector|MakeVector (* _index_2 (/ (.x (- (Variables|Default|GetTopRightGridLocation) (Variables|Default|GetBottomLeftGridLocation))) (Math|Conversions|ToFloat(Integer) (- (Variables|Default|GetNumberOfGridTiles_X) 1)))) (* _index (/ (.y (- (Variables|Default|GetTopRightGridLocation) (Variables|Default|GetBottomLeftGridLocation))) (Math|Conversions|ToFloat(Integer) (- (Variables|Default|GetNumberOfGridTiles_Y) 1)))) 0.0)))))))
  (for (_array_element _array_index) (Variables|Default|GetGrid)
    (for (_array_element_2 _array_index_2) (Utilities|Struct|BreakFGridCols _array_element)
      (bind _returnvalue_4 (Game|SpawnActorfromClass "/Game/Blueprints/Rooms/TestUnit.TestUnit_C" (Math|Transform|MakeTransform _array_element_2 "0, 0, 0" "1,1,1") "Undefined" 0 0)))))

(event Custom|PlayerChangedRoom
  ;[1 1 1] PlayerChangedRoom
  (if (not (Variables|Default|GetRoomEnteredBefore)) ; True - The room has already been entered, \nFalse - A new room has been entered
    (CallFunction|PopulateRoom (.RoomLayout (Utilities|Struct|BreakFRoomInfo (Variables|Default|GetRoomInfo))))
    (CallFunction|SetPlayerCurrentRoomtoSelf)))

(event EventBeginPlay
  (bind _defaultsceneroot (Variables|Default|GetDefaultSceneRoot))
  (bind _defaultsceneroot_2 (Variables|Default|GetDefaultSceneRoot))
  (bind _defaultsceneroot_3 (Variables|Default|GetDefaultSceneRoot))
  (bind _defaultsceneroot_4 (Variables|Default|GetDefaultSceneRoot))
  (bind _returnvalue (Transformation|GetWorldTransform _defaultsceneroot_2))
  (bind _returnvalue_2 (Transformation|GetWorldTransform _defaultsceneroot_3))
  (bind _returnvalue_3 (Transformation|GetWorldTransform _defaultsceneroot))
  (bind _returnvalue_4 (Transformation|GetWorldTransform _defaultsceneroot_4))
  ;[1 1 1] BeginPlay / Spawn Doors
  (if (Variables|Default|GetIsSpawnRoom)
    (Variables|Default|SetRoomEnteredBefore true)
    (bind _astwin_stick_mode (Utilities|Casting|CastToTwinStickMode (Game|GetGameMode)))
    (Variables|/Game/Blueprints/TwinStickMode.TwinStickMode_C|SetSpawnRoom _astwin_stick_mode self))
  (Variables|Default|SetTopRightCornerOfFloor (CallFunction|GetTopRightCornerOfFloor))
  (CallFunction|CreateGridUnits)
  (Variables|Default|SetY_WestWall%20&%20X_SouthWall -950)
  (Variables|Default|SetY_EastWall%20&%20X_NorthWall 950)
  (Variables|Default|SetRotate 90)
  (bind _returnvalue_5 (Game|SpawnActorfromClass "/Game/Blueprints/Rooms/Door.Door_C" (Math|Transform|MakeTransform (Math|Vector|MakeVector (.x (.location _returnvalue_3)) (+ (.y (.location _returnvalue_3)) (Math|Conversions|ToFloat(Integer) (Variables|Default|GetY_EastWall%20&%20X_NorthWall))) (+ (.z (.location _returnvalue_3)) (Math|Conversions|ToFloat(Integer) (Variables|Default|GetZ_Floor)))) "0, 0, 0" "1,1,1") "Undefined" 0 0))
  (Variables|Default|SetEastDoor _returnvalue_5)
  (bind _returnvalue_6 (Game|SpawnActorfromClass "/Game/Blueprints/Rooms/Door.Door_C" (Math|Transform|MakeTransform (Math|Vector|MakeVector (.x (.location _returnvalue_2)) (+ (.y (.location _returnvalue_2)) (Math|Conversions|ToFloat(Integer) (Variables|Default|GetY_WestWall%20&%20X_SouthWall))) (+ (.z (.location _returnvalue_2)) (Math|Conversions|ToFloat(Integer) (Variables|Default|GetZ_Floor)))) "0, 0, 0" "1,1,1") "Undefined" 0 0))
  (Variables|Default|SetWestDoor _returnvalue_6)
  (bind _returnvalue_7 (Game|SpawnActorfromClass "/Game/Blueprints/Rooms/Door.Door_C" (Math|Transform|MakeTransform (Math|Vector|MakeVector (+ (.x (.location _returnvalue_4)) (Math|Conversions|ToFloat(Integer) (Variables|Default|GetY_WestWall%20&%20X_SouthWall))) (.y (.location _returnvalue_4)) (+ (.z (.location _returnvalue_4)) (Math|Conversions|ToFloat(Integer) (Variables|Default|GetZ_Floor)))) (Math|Rotator|MakeRotator (.roll (.rotation _returnvalue_4)) (.pitch (.rotation _returnvalue_4)) (+ (.yaw (.rotation _returnvalue_4)) (Math|Conversions|ToFloat(Integer) (Variables|Default|GetRotate)))) "1,1,1") "Undefined" 0 0))
  (Variables|Default|SetSouthDoor _returnvalue_7)
  (bind _returnvalue_8 (Game|SpawnActorfromClass "/Game/Blueprints/Rooms/Door.Door_C" (Math|Transform|MakeTransform (Math|Vector|MakeVector (+ (.x (.location _returnvalue)) (Math|Conversions|ToFloat(Integer) (Variables|Default|GetY_EastWall%20&%20X_NorthWall))) (.y (.location _returnvalue)) (+ (.z (.location _returnvalue)) (Math|Conversions|ToFloat(Integer) (Variables|Default|GetZ_Floor)))) (Math|Rotator|MakeRotator (.roll (.rotation _returnvalue)) (.pitch (.rotation _returnvalue)) (+ (.yaw (.rotation _returnvalue)) (Math|Conversions|ToFloat(Integer) (Variables|Default|GetRotate)))) "1,1,1") "Undefined" 0 0))
  (Variables|Default|SetNorthDoor _returnvalue_8)
  (if (Variables|Default|GetIsSpawnRoom)
    (CallFunction|PopulateRoom (.RoomLayout (Utilities|Struct|BreakFRoomInfo (Variables|Default|GetRoomInfo))))))

(event Collision|EventActorBeginOverlap
  (params (OtherActor :type Actor%20Object%20Reference))
  (bind _defaultsceneroot (Variables|Default|GetDefaultSceneRoot))
  (bind _returnvalue (Transformation|GetWorldLocation _defaultsceneroot))
  ;[1 1 1] Camera switch to appropriate room
  (if (Utilities|IsValid OtherActor)
    (if (Actor|ActorHasTag OtherActor "Projectile")
      (bind _asprojectile (Utilities|Casting|CastToProjectile OtherActor))
      (Default|DestroywithSparks _asprojectile)
      (elif (Actor|ActorHasTag OtherActor "Friendly")
        (CallFunction|PlayerChangedRoom)
        (Variables|Default|SetRoomEnteredBefore true)
        (bind _astwin_stick_mode (Utilities|Casting|CastToTwinStickMode (Game|GetGameMode)))
        (Transformation|SetWorldLocation (Variables|/Script/Engine.Actor|GetRootComponent (Variables|/Game/Blueprints/TwinStickMode.TwinStickMode_C|GetCameraReference _astwin_stick_mode)) (Math|Vector|MakeVector (.x _returnvalue) (.y _returnvalue) (+ (.z _returnvalue) 2e+03)) false false)))))

(event EventTick
  (params (DeltaSeconds :type Float%20%28single-precision%29))
  ;[1 1 1] To destroy appropriate doors
  (if (Variables|Default|GetRoomEnteredBefore)
    (if (== (Variables|Default|GetCurrentEnemyCount) 0)
      (Utilities|FlowControl|DoOnce false
        (:Completed
          (switch Utilities|FlowControl|Switch|SwitchonERoomDoorType (.DoorsToOpen (Utilities|Struct|BreakFRoomInfo (Variables|Default|GetRoomInfo)))
            (:NewEnumerator7
              (Actor|DestroyActor (Variables|Default|GetNorthDoor) :!label _label))
            (:NewEnumerator8
              (Utilities|FlowControl|Sequence
                (:then_0
                  (goto _label))
                (:then_1
                  (Actor|DestroyActor (Variables|Default|GetEastDoor) :!label _label_2))))
            (:NewEnumerator10
              (Utilities|FlowControl|Sequence
                (:then_0
                  (goto _label))
                (:then_1
                  (Actor|DestroyActor (Variables|Default|GetSouthDoor) :!label _label_3))))
            (:NewEnumerator17
              (Utilities|FlowControl|Sequence
                (:then_0
                  (goto _label))
                (:then_1
                  (Actor|DestroyActor (Variables|Default|GetWestDoor) :!label _label_4))))
            (:NewEnumerator9
              (Utilities|FlowControl|Sequence
                (:then_0
                  (goto _label))
                (:then_1
                  (goto _label_2))
                (:then_2
                  (goto _label_3))))
            (:NewEnumerator11
              (Utilities|FlowControl|Sequence
                (:then_0
                  (goto _label))
                (:then_1
                  (goto _label_4))
                (:then_2
                  (goto _label_3))))
            (:NewEnumerator12
              (goto _label_3))
            (:NewEnumerator13
              (Utilities|FlowControl|Sequence
                (:then_0
                  (goto _label_3))
                (:then_1
                  (goto _label_2))))
            (:NewEnumerator6
              (goto _label_2))
            (:NewEnumerator14
              (goto _label_4))))))))

(fn ConstructionScript)

(fn GetDistanceBetweenGridUnitsY
  (params (GridUnit :type Test%20Unit%20Object%20Reference))
  (return (+ 0.0 (/ (- (* (.y (.BoxExtent (Collision|GetComponentBounds (Variables|Default|Getfloor)))) 2.0) 0.0) (Math|Conversions|ToFloat(Integer) (Variables|Default|GetNumberOfGridTiles_Y))))))

(fn GetWallThickness
  (return (* (.y (.BoxExtent (Collision|GetComponentBounds (Variables|Default|GetTWall1)))) 2.0)))

(fn GetTopRightCornerOfRoom
  (params (GridUnit :type Actor%20Object%20Reference))
  (bind _wallthickness (CallFunction|GetWallThickness))
  (bind _floor (Variables|Default|Getfloor))
  (bind _rootcomponent (Variables|/Script/Engine.Actor|GetRootComponent GridUnit))
  (bind (_origin _boxextent) (Collision|GetComponentBounds _rootcomponent))
  (bind (_origin_2 _boxextent_2) (Collision|GetComponentBounds _floor))
  (bind _returnvalue (+ _origin _boxextent))
  (return (Math|Vector|MakeVector (- (.x _returnvalue) _wallthickness) (- (.y _returnvalue) _wallthickness) (+ (.z _origin_2) (.z _boxextent_2)))))

(fn GetBottomLeftCornerOfRoom
  (params (GridUnit :type Actor%20Object%20Reference))
  (bind _wallthickness (CallFunction|GetWallThickness))
  (bind _rootcomponent (Variables|/Script/Engine.Actor|GetRootComponent GridUnit))
  (bind _floor (Variables|Default|Getfloor))
  (bind _boxextent (Collision|GetComponentBounds _rootcomponent))
  (bind (_origin _boxextent_2) (Collision|GetComponentBounds _floor))
  (bind _returnvalue (- _origin _boxextent_2))
  (return (Math|Vector|MakeVector (+ (.x _boxextent) (+ (.x _returnvalue) _wallthickness)) (+ (.y _boxextent) (+ (.y _returnvalue) _wallthickness)) (.z (+ _origin _boxextent_2)))))

(fn GetGridTileLocation
  (params (x :type Integer) (Y :type Integer))
  (return (Utilities|Array|Get(acopy) (Utilities|Struct|BreakFGridCols (Utilities|Array|Get(acopy) (Variables|Default|GetGrid) (- (- (Variables|Default|GetNumberOfGridTiles_X) 1) x))) (- (- (Variables|Default|GetNumberOfGridTiles_Y) 1) Y))))

(fn PopulateRoom
  (params (RoomLayout :type ERoomLayout%20Enum :default "NewEnumerator0"))
  (bind _returnvalue (Utilities|GetDataTableRow "/Game/Blueprints/SpreadSheet_Interaction/Rooms/DT_RoomLayouts.DT_RoomLayouts" (Utilities|String|StringToName (Utilities|String|EnumtoString RoomLayout)))
    (:then
      (bind _output_get (Variables|Default|SetRoomLayout _returnvalue))
      (for _array_element (Utilities|Struct|BreakFRoomLayout _output_get)
        (bind _location (CallFunction|GetGridTileLocation (.X-Coordinate (Utilities|Struct|BreakFGridUnit _array_element)) (.Y-Coordinate (Utilities|Struct|BreakFGridUnit _array_element))))
        (switch Utilities|FlowControl|Switch|SwitchonEGridTileType (.TileType (Utilities|Struct|BreakFGridUnit _array_element))
          (:NewEnumerator2
            (Game|SpawnActorfromClass "/Game/Blueprints/Rooms/TestUnit.TestUnit_C" (Math|Transform|MakeTransform _location "0, 0, 0" "1,1,4.000000") "Undefined" 0 0))
          (:NewEnumerator1
            (CallFunction|SpawnEnemy _location (.TileType (Utilities|Struct|BreakFGridUnit _array_element)) :!label _label)
            (Math|Integer|IncrementInt (Variables|Default|GetCurrentEnemyCount)))
          (:NewEnumerator3
            (goto _label))
          (:NewEnumerator4
            (goto _label))
          (:NewEnumerator5
            (goto _label))
          (:NewEnumerator6
            (goto _label))
          (:NewEnumerator7
            (goto _label))
          (:NewEnumerator10
            (Game|SpawnActorfromClass "/Game/Blueprints/Rooms/TestUnit.TestUnit_C" (Math|Transform|MakeTransform _location "0, 0, 0" "4.500000,4.500000,3.000000") "Undefined" 0 0))))
      (Variables|Default|SetInitialEnemyCount (Variables|Default|GetCurrentEnemyCount)))
    (:RowNotFound
      (Development|PrintString "Row Not Found: Room Layout"))))

(fn SpawnEnemy
  (params (Location :type Vector) (GridTile :type EGridTileType%20Enum :default "NewEnumerator0"))
  (Utilities|FlowControl|Sequence
    (:then_0
      (switch Utilities|FlowControl|Switch|SwitchonEGridTileType GridTile
        (:NewEnumerator1
          (Variables|Default|SetEnemyType "NewEnumerator0"))
        (:NewEnumerator3
          (Variables|Default|SetEnemyType "NewEnumerator1"))
        (:NewEnumerator4
          (Variables|Default|SetEnemyType "NewEnumerator3"))
        (:NewEnumerator5
          (Variables|Default|SetEnemyType "NewEnumerator2"))
        (:NewEnumerator6
          (Variables|Default|SetEnemyType "NewEnumerator4"))
        (:NewEnumerator7
          (Variables|Default|SetEnemyType "NewEnumerator5"))))
    (:then_1
      (bind _returnvalue (AI|SpawnAIFromClass "/Game/Blueprints/Enemies/EnemyCharacter.EnemyCharacter_C" 0 Location "0, 0, 0" false))
      (bind _asenemy_character (Utilities|Casting|CastToEnemyCharacter _returnvalue))
      (bind _output_get (Variables|/Game/Blueprints/Enemies/EnemyCharacter.EnemyCharacter_C|SetcurrentRoom _asenemy_character self))
      (Utilities|Array|Add (Variables|Room_C|GetEnemiesInTheRoom _output_get) _asenemy_character)
      (Default|ChangeEnemyType _asenemy_character (Variables|Default|GetEnemyType)))))

(fn GetTopRightCornerOfFloor
  (bind _wallthickness (CallFunction|GetWallThickness))
  (bind _floor (Variables|Default|Getfloor))
  (bind (_origin _boxextent) (Collision|GetComponentBounds _floor))
  (bind _returnvalue (* _wallthickness 1.0))
  (return (+ _origin (Math|Vector|MakeVector (- (.x _boxextent) _returnvalue) (- (.y _boxextent) _returnvalue) (.z _boxextent)))))

(fn SetPlayerCurrentRoomtoSelf
  (bind _astwin_stick_mode (Utilities|Casting|CastToTwinStickMode (Game|GetGameMode)))
  (Variables|/Game/Blueprints/HeroCharacter.HeroCharacter_C|SetCurrentRoom (Variables|/Game/Blueprints/TwinStickMode.TwinStickMode_C|GetPlayerReference _astwin_stick_mode) self))