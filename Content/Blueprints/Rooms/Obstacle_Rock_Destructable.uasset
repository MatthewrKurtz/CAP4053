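; Destructible rock obstacle for rooms that breaks when its health runs out and can leave an item behind.
; AffectHealth adds a signed delta to Health, so damage arrives as a negative value.
; At zero or below, a one-in-ten roll spawns a BP_BaseItem at the rock's transform and sets it to the rock's ItemType, then the rock destroys itself.
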(event EventAffectHealth
  (params (Delta :type Float%20%28single-precision%29))
  (Variables|Default|SetHealth (+ Delta (Variables|Default|GetHealth)))
  (if (<= (Variables|Default|GetHealth) 0.0)
    (Utilities|FlowControl|Sequence
      (:then_0
        (if (<= (Math|Random|RandomFloat) 0.1)
          (bind _returnvalue (Game|SpawnActorfromClass "/Game/Blueprints/Interactables/BP_BaseItem.BP_BaseItem_C" (Transformation|GetActorTransform self) "Undefined" 0 0))
          (Default|ChangeItemType _returnvalue (Variables|Default|GetItemType))))
      (:then_1
        (Actor|DestroyActor)))))

(fn ConstructionScript
  (|CallParentFunction))