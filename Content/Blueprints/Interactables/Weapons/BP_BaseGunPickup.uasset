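; BP_BaseGunPickup is a base gun Blueprint that spawns projectiles repeatedly while its trigger is held.
; PullTrigger fires immediately, then starts a looping timer at RoundsPerSecond, with a DoOnce guard that ReleaseTrigger resets as it clears the timer.
; Each shot spawns ProjectileType at ProjectileSpawnPoint, with ChangeWeaponSpread randomizing only the yaw within SpreadAmount either way.
; The file contains no pickup or overlap logic.
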(event Custom|PullTrigger
  ;[1 1 1] Fire in Rounds Per Second When Trigger is Pulled/Released
  (Utilities|FlowControl|DoOnce false
    (:Completed
      (CallFunction|Fire)
      (Utilities|Time|SetTimerbyFunctionName 0 "Fire" (/ 1.0 (Variables|Default|GetRoundsPerSecond)) true))))

(event Custom|ReleaseTrigger
  ;[1 1 1] Fire in Rounds Per Second When Trigger is Pulled/Released
  (Utilities|Time|ClearTimerbyFunctionName 0 "Fire")
  (Utilities|FlowControl|DoOnce false) ; enters at Reset
)

(event Custom|Fire
  ;[1 1 1] Fire (Spawn Projectile)
  (Game|SpawnActorfromClass (Variables|Default|GetProjectileType) (CallFunction|ChangeWeaponSpread (Variables|Default|GetSpreadAmount)) "Undefined" 0 0))

(event EventBeginPlay
  (|CallParentFunction) ; This node is disabled and will not be called.\nDrag off pins to build functionality.
)

(event Collision|EventActorBeginOverlap
  (params (OtherActor :type Actor%20Object%20Reference))
  (|CallParentFunction OtherActor) ; This node is disabled and will not be called.\nDrag off pins to build functionality.
)

(event EventTick
  (params (DeltaSeconds :type Float%20%28single-precision%29))
  (|CallParentFunction DeltaSeconds) ; This node is disabled and will not be called.\nDrag off pins to build functionality.
)

(fn ConstructionScript
  (|CallParentFunction))

(fn ChangeWeaponSpread
  (params (SpreadAmount :type Float%20%28single-precision%29))
  (bind _projectilespawnpoint (Variables|Default|GetProjectileSpawnPoint))
  (bind _returnvalue (Transformation|GetWorldTransform _projectilespawnpoint))
  (return (Math|Transform|MakeTransform (.location _returnvalue) (Math|Rotator|MakeRotator (.roll (.rotation _returnvalue)) (.pitch (.rotation _returnvalue)) (+ (.yaw (.rotation _returnvalue)) (Math|Random|RandomFloatinRange SpreadAmount (* SpreadAmount -1.0)))) (.scale _returnvalue))))