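; Trident shot weapon pickup whose Fire event launches three projectiles in a fan.
; It spawns one ProjectileType actor along the aim transform and two more with yaw offset by plus and minus AngleBetweenShots.
; Each spawn takes its transform from ChangeWeaponSpread using SpreadAmount.
; The construction script only calls the parent's.
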(event Custom|Fire
  (bind _spreadamount (Variables|Default|GetSpreadAmount))
  (bind _projectiletype (Variables|Default|GetProjectileType))
  (bind _anglebetweenshots (Variables|Default|GetAngleBetweenShots))
  (bind _spawntransform (CallFunction|ChangeWeaponSpread _spreadamount))
  (bind (_roll _pitch _yaw) (Math|Rotator|BreakRotator (.rotation _spawntransform)))
  (Game|SpawnActorfromClass _projectiletype (Math|Transform|MakeTransform (.location _spawntransform) (.rotation _spawntransform) (.scale _spawntransform)) "Undefined" 0 0)
  (Game|SpawnActorfromClass _projectiletype (Math|Transform|MakeTransform (.location _spawntransform) (Math|Rotator|MakeRotator _roll _pitch (+ _yaw _anglebetweenshots)) (.scale _spawntransform)) "Undefined" 0 0)
  (Game|SpawnActorfromClass _projectiletype (Math|Transform|MakeTransform (.location _spawntransform) (Math|Rotator|MakeRotator _roll _pitch (- _yaw _anglebetweenshots)) (.scale _spawntransform)) "Undefined" 0 0))

(fn ConstructionScript
  (|CallParentFunction))