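; BP_BaseItem is the base interactable item actor that players pick up into their inventory.
; On BeginPlay it looks up its ItemType enum, converted to a row name, in DT_Items and caches the row as ItemInfo.
; On Interaction, if the instigator has inventory space, it sends ItemInfo through PickupMessage and destroys itself.
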(event EventInteraction
  (params (Instigator :type Hero%20Character%20Object%20Reference))
  (if (Default|HasSpaceinInventory Instigator)
    (Class|BPIInteract|Pickup(Message) Instigator (Variables|Default|GetItemInfo))
    (Actor|DestroyActor)))

(event EventBeginPlay
  (CallFunction|ChangeItemType (Variables|Default|GetItemType)))

(fn ConstructionScript
  (|CallParentFunction))

(fn ChangeItemType
  (params (NewItemType :type EItems_Specific%20Enum :default "NewEnumerator0"))
  (bind _returnvalue (Utilities|GetDataTableRow "/Game/Blueprints/SpreadSheet_Interaction/Items/DT_Items.DT_Items" (Utilities|String|StringToName (Utilities|String|EnumtoString NewItemType)))
    (:then
      (Variables|Default|SetItemInfo _returnvalue))))