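; Room actor for a twin-stick game that spawns four wall doors and one enemy at BeginPlay.
; Overlap by a "Friendly"-tagged actor moves the game mode's camera above the room's center.
; The enemy receives a room reference; DecrementCount lowers the enemy count, and Tick destroys the room actor once it reaches zero, leaving the spawned doors.
; Neighbor detection and door-removal logic sits disconnected and never runs.
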(event Custom|Decrement%20Count
  (bind _result (Math|Integer|DecrementInt (Variables|Default|GetCount))
    (:%20%20
      (Variables|Default|SetCount _result))))

(event EventBeginPlay
  (bind _defaultsceneroot (Variables|Default|GetDefaultSceneRoot))
  (bind _defaultsceneroot_2 (Variables|Default|GetDefaultSceneRoot))
  (bind _defaultsceneroot_3 (Variables|Default|GetDefaultSceneRoot))
  (bind _defaultsceneroot_4 (Variables|Default|GetDefaultSceneRoot))
  (bind _defaultsceneroot_5 (Variables|Default|GetDefaultSceneRoot))
  (bind _returnvalue (Transformation|GetWorldTransform _defaultsceneroot_2))
  (bind _returnvalue_2 (Transformation|GetWorldTransform _defaultsceneroot_3))
  (bind _returnvalue_3 (Transformation|GetWorldTransform _defaultsceneroot))
  (bind _returnvalue_4 (Transformation|GetWorldTransform _defaultsceneroot_4))
  (bind _returnvalue_5 (Transformation|GetWorldTransform _defaultsceneroot_5))
  (Variables|Default|SetZ_Floor 50)
  (Variables|Default|SetY_WestWall%20&%20X_SouthWall -950)
  (Variables|Default|SetY_EastWall%20&%20X_NorthWall 950)
  (Variables|Default|SetRotate 90)
  (bind _returnvalue_6 (Game|SpawnActorfromClass "/Game/Blueprints/RoomFolder/Door.Door_C" (Math|Transform|MakeTransform (Math|Vector|MakeVector (.x (.location _returnvalue_3)) (+ (.y (.location _returnvalue_3)) (Math|Conversions|ToFloat(Integer) (Variables|Default|GetY_EastWall%20&%20X_NorthWall))) (+ (.z (.location _returnvalue_3)) (Math|Conversions|ToFloat(Integer) (Variables|Default|GetZ_Floor)))) "0, 0, 0" "1,1,1") "Undefined" 0 0))
  (Variables|Default|SetEast _returnvalue_6)
  (bind _returnvalue_7 (Game|SpawnActorfromClass "/Game/Blueprints/RoomFolder/Door.Door_C" (Math|Transform|MakeTransform (Math|Vector|MakeVector (.x (.location _returnvalue_2)) (+ (.y (.location _returnvalue_2)) (Math|Conversions|ToFloat(Integer) (Variables|Default|GetY_WestWall%20&%20X_SouthWall))) (+ (.z (.location _returnvalue_2)) (Math|Conversions|ToFloat(Integer) (Variables|Default|GetZ_Floor)))) "0, 0, 0" "1,1,1") "Undefined" 0 0))
  (Variables|Default|SetWest _returnvalue_7)
  (bind _returnvalue_8 (Game|SpawnActorfromClass "/Game/Blueprints/RoomFolder/Door.Door_C" (Math|Transform|MakeTransform (Math|Vector|MakeVector (+ (.x (.location _returnvalue_4)) (Math|Conversions|ToFloat(Integer) (Variables|Default|GetY_WestWall%20&%20X_SouthWall))) (.y (.location _returnvalue_4)) (+ (.z (.location _returnvalue_4)) (Math|Conversions|ToFloat(Integer) (Variables|Default|GetZ_Floor)))) (Math|Rotator|MakeRotator (.roll (.rotation _returnvalue_4)) (.pitch (.rotation _returnvalue_4)) (+ (.yaw (.rotation _returnvalue_4)) (Math|Conversions|ToFloat(Integer) (Variables|Default|GetRotate)))) "1,1,1") "Undefined" 0 0))
  (Variables|Default|SetSouth _returnvalue_8)
  (bind _returnvalue_9 (Game|SpawnActorfromClass "/Game/Blueprints/RoomFolder/Door.Door_C" (Math|Transform|MakeTransform (Math|Vector|MakeVector (+ (.x (.location _returnvalue)) (Math|Conversions|ToFloat(Integer) (Variables|Default|GetY_EastWall%20&%20X_NorthWall))) (.y (.location _returnvalue)) (+ (.z (.location _returnvalue)) (Math|Conversions|ToFloat(Integer) (Variables|Default|GetZ_Floor)))) (Math|Rotator|MakeRotator (.roll (.rotation _returnvalue)) (.pitch (.rotation _returnvalue)) (+ (.yaw (.rotation _returnvalue)) (Math|Conversions|ToFloat(Integer) (Variables|Default|GetRotate)))) "1,1,1") "Undefined" 0 0))
  (Variables|Default|SetNorth _returnvalue_9)
  (bind _returnvalue_10 (Game|SpawnActorfromClass "/Game/Blueprints/EnemyCharacter.EnemyCharacter_C" (Math|Transform|MakeTransform (Math|Vector|MakeVector (.x (.location _returnvalue_5)) (.y (.location _returnvalue_5)) (+ (.z (.location _returnvalue_5)) (Math|Conversions|ToFloat(Integer) (Variables|Default|GetZ_Floor)))) (.rotation _returnvalue_5) (.scale _returnvalue_5)) "Undefined" 0 0))
  (bind _result (Math|Integer|IncrementInt (Variables|Default|GetCount))
    (:%20%20
      (Variables|Default|SetCount _result)
      (Variables|/Game/Blueprints/EnemyCharacter.EnemyCharacter_C|SetCurrent%20Room _returnvalue_10 self))))

(event Collision|EventActorBeginOverlap
  (params (OtherActor :type Actor%20Object%20Reference))
  (bind _defaultsceneroot (Variables|Default|GetDefaultSceneRoot))
  (bind _returnvalue (Transformation|GetWorldLocation _defaultsceneroot))
  (if (Actor|ActorHasTag OtherActor "Friendly")
    (bind _astwin_stick_mode (Utilities|Casting|CastToTwinStickMode (Game|GetGameMode)))
    (Transformation|SetWorldLocation (Variables|/Script/Engine.Actor|GetRootComponent (Variables|/Game/Blueprints/TwinStickMode.TwinStickMode_C|GetCameraReference _astwin_stick_mode)) (Math|Vector|MakeVector (.x _returnvalue) (.y _returnvalue) (+ (.z _returnvalue) 2e+03)) false false)))

(event EventTick
  (params (DeltaSeconds :type Float%20%28single-precision%29))
  (if (== (Variables|Default|GetCount) 0)
    (Utilities|FlowControl|DoOnce false
      (:Completed
        (Actor|DestroyActor)))))

(fn ConstructionScript)