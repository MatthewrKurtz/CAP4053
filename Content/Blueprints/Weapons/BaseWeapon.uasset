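; Base weapon Blueprint that fires projectiles automatically while the trigger is held.
; On BeginPlay it loads WeaponInfo from the hardcoded AssaultRifle row of DT_Weapons.
; PullTrigger fires immediately and starts a looping timer at RoundsPerSecond, guarded by a DoOnce that ReleaseTrigger resets while clearing the timer.
; Each shot maps the projectile type to a class, spawns it at ProjectileSpawnPoint with random yaw-only spread, and increments NumberOfBulletsFired.
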(event Custom|PullTrigger
  ;[1 1 1] Fire in Rounds Per Second When Trigger is Pulled/Released
  (Utilities|FlowControl|DoOnce false
    (:Completed
      (CallFunction|Fire)
      (Utilities|Time|SetTimerbyFunctionName 0 "Fire" (/ 1.0 (Variables|Default|GetRoundsPerSecond)) true))))

(event Custom|ReleaseTrigger
  ;[1 1 1] Fire in Rounds Per Second When Trigger is Pulled/Released
  (Utilities|Time|ClearTimerbyFunctionName 0 "Fire")
  (Utilities|FlowControl|DoOnce false) ; enters at Reset
)

(event Custom|Fire
  (bind _weaponinfo (Variables|Default|GetWeaponInfo))
  (bind (_projectiletype _spread) (Utilities|Struct|BreakFWeaponInfo _weaponinfo))
  ;[1 1 1] Fire (Spawn Projectile)
  (CallFunction|SpawnProjectile _projectiletype _spread))

(event EventBeginPlay
  (bind _returnvalue (Utilities|GetDataTableRow "/Game/Blueprints/SpreadSheet_Interaction/Weapons/DT_Weapons.DT_Weapons" "AssaultRifle")
    (:then
      (Variables|Default|SetWeaponInfo _returnvalue))
    (:RowNotFound
      (Development|PrintString "Row Not Found: Base Weapon"))))

(fn ConstructionScript)

(fn ChangeWeaponSpread
  (params (Spread%20Amount :type Float%20%28single-precision%29))
  (bind _projectilespawnpoint (Variables|Default|GetProjectileSpawnPoint))
  (bind _returnvalue (Transformation|GetWorldTransform _projectilespawnpoint))
  (return (Math|Transform|MakeTransform (.location _returnvalue) (Math|Rotator|MakeRotator (.roll (.rotation _returnvalue)) (.pitch (.rotation _returnvalue)) (+ (.yaw (.rotation _returnvalue)) (Math|Random|RandomFloatinRange Spread%20Amount (* Spread%20Amount -1.0)))) (.scale _returnvalue))))

(fn SpawnProjectile
  (params (Projectile%20Type :type EProjectileType%20Enum :default "NewEnumerator0") (Spread%20Amount :type Float%20%28single-precision%29))
  (bind _projectile_class (CallFunction|GetProjectileClass Projectile%20Type))
  (Game|SpawnActorfromClass _projectile_class (CallFunction|ChangeWeaponSpread Spread%20Amount) "Undefined" 0 0)
  (Math|Integer|IncrementInt (Variables|Default|GetNumberOfBulletsFired)))

(fn GetProjectileClass
  (params (Selection :type EProjectileType%20Enum :default "NewEnumerator0"))
  (switch Utilities|FlowControl|Switch|SwitchonEProjectileType Selection
    (:NewEnumerator0
      (return "/Game/Blueprints/Weapons/Projectile.Projectile_C"))
    (:NewEnumerator1
      (return "/Game/Blueprints/Weapons/Projectile_ChargeShot.Projectile_ChargeShot_C"))
    (:NewEnumerator2
      (return "/Game/Blueprints/Weapons/Projectile_Homing.Projectile_Homing_C"))
    (:NewEnumerator3
      (return "/Game/Blueprints/Weapons/Projectile_Enemy.Projectile_Enemy_C"))
    (:NewEnumerator4
      (return "/Game/Blueprints/Weapons/Projectile_Pellet.Projectile_Pellet_C"))))