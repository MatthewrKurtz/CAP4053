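; Charge shot weapon Blueprint that fires projectiles after the trigger has been held for the weapon's attack interval.
; BeginPlay loads its stats from the ChargeShot row of DT_Weapons.
; PullTrigger starts a real-time timer through a DoOnce, which ReleaseTrigger resets while stopping fire.
; Tick spawns a projectile with the table's type and spread each time the interval elapses, restarting the timer so shots repeat while held.
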(event EventBeginPlay
  (bind _returnvalue (Utilities|GetDataTableRow "/Game/Blueprints/SpreadSheet_Interaction/DT_Weapons.DT_Weapons" "ChargeShot")
    (:then
      (Variables|Default|SetWeaponInfo _returnvalue))
    (:RowNotFound
      (Development|PrintString "Row Not Found: ChargeShot"))))

(event EventPullTrigger
  (Utilities|FlowControl|DoOnce false
    (:Completed
      (Variables|Default|SetStartFire (Utilities|Time|GetRealTimeSeconds))
      (Variables|Default|SetFire_0 true))))

(event EventTick
  (params (DeltaSeconds :type Float%20%28single-precision%29))
  (bind _weaponinfo (Variables|Default|GetWeaponInfo))
  (bind (_projectiletype _spread _attackspeed) (Utilities|Struct|BreakFWeaponInfo _weaponinfo))
  (if (and (> (- (Utilities|Time|GetRealTimeSeconds) (Variables|Default|GetStartFire)) _attackspeed) (Variables|Default|GetFire_0))
    (Variables|Default|SetStartFire (Utilities|Time|GetRealTimeSeconds))
    (CallFunction|SpawnProjectile _projectiletype _spread)))

(event EventReleaseTrigger
  (Variables|Default|SetFire_0 false)
  (Utilities|FlowControl|DoOnce false) ; enters at Reset
)

(fn ConstructionScript
  (|CallParentFunction))