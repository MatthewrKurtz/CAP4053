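; Shotgun weapon Blueprint that fires several pellet projectiles per shot.
; On BeginPlay it loads the Shotgun row from DT_Weapons into WeaponInfo and resolves the projectile class from its projectile type.
; PullTrigger rate-limits shots by comparing real time since the last shot to AttackSpeed.
; Fire spawns one projectile per pellet, each with its own transform from ChangeWeaponSpread using the weapon's spread.
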(event EventBeginPlay
  (bind _returnvalue (Utilities|GetDataTableRow "/Game/Blueprints/SpreadSheet_Interaction/DT_Weapons.DT_Weapons" "Shotgun")
    (:then
      (Variables|Default|SetWeaponInfo _returnvalue)
      (bind _projectile_class (CallFunction|GetProjectileClass (.ProjectileType (Utilities|Struct|BreakFWeaponInfo _returnvalue))))
      (Variables|Default|SetProjectileClass _projectile_class))))

(event EventFire
  (Variables|Default|SetTimeLastFired (Utilities|Time|GetRealTimeSeconds))
  (for _index (range 0 (- (Variables|Default|GetNumberOfPellets) 1))
    (Game|SpawnActorfromClass (Variables|Default|GetProjectileClass) (CallFunction|ChangeWeaponSpread (Utilities|Struct|BreakFWeaponInfo (Variables|Default|GetWeaponInfo))) "Undefined" 0 0)))

(event EventPullTrigger
  (if (> (- (Utilities|Time|GetRealTimeSeconds) (Variables|Default|GetTimeLastFired)) (Utilities|Struct|BreakFWeaponInfo (Variables|Default|GetWeaponInfo)))
    (CallFunction|Fire)))

(fn ConstructionScript
  (|CallParentFunction)
  (Variables|Default|SetWeaponInfo (Utilities|Struct|MakeFWeaponInfo "NewEnumerator0" "NewEnumerator0" 0.0 0.0 0.0 0.0 0 0 0 0 0)))