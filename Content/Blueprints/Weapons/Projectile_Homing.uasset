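; Homing projectile for a twin-stick shooter that locks onto a nearby enemy when it spawns.
; On BeginPlay it plays a laser sound through the game mode's audio manager, then scans all EnemyCharacter actors for the closest damage volume within the running ShortestLength threshold.
; If one is found, that enemy's root component becomes the ProjectileMovement homing target, chosen once and never re-evaluated.
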(event EventBeginPlay
  (bind _astwin_stick_mode (Utilities|Casting|CastToTwinStickMode (Game|GetGameMode)))
  (Default|LaserSound4 (Variables|/Game/Blueprints/TwinStickMode.TwinStickMode_C|GetAudioManagerReference _astwin_stick_mode))
  (bind _outactors (Actor|GetAllActorsOfClass "/Game/Blueprints/Enemies/EnemyCharacter.EnemyCharacter_C"))
  (for _array_element _outactors
    (if (<= (Math|Vector|VectorLength (- (.location (Transformation|GetWorldTransform (Variables|/Game/Blueprints/Enemies/EnemyCharacter.EnemyCharacter_C|GetDamageVolume _array_element))) (.location (Transformation|GetWorldTransform (Variables|Default|GetDefaultSceneRoot))))) (Variables|Default|GetShortestLength))
      (Variables|Default|SetShortestLength (Math|Vector|VectorLength (- (.location (Transformation|GetWorldTransform (Variables|/Game/Blueprints/Enemies/EnemyCharacter.EnemyCharacter_C|GetDamageVolume _array_element))) (.location (Transformation|GetWorldTransform (Variables|Default|GetDefaultSceneRoot))))))
      (Variables|Default|SetClosestEnemy _array_element)))
  (Utilities|IsValid (Variables|Default|GetClosestEnemy)
    (:Is%20Valid
      (Variables|/Script/Engine.ProjectileMovementComponent|SetHomingTargetComponent (Variables|Default|GetProjectileMovement) (Variables|/Script/Engine.Actor|GetRootComponent (Variables|Default|GetClosestEnemy))))))

(fn ConstructionScript
  (|CallParentFunction))