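; Projectile Blueprint for a twin-stick game that damages what it overlaps, playing laser and hit sounds through the game mode's audio manager.
; Walls destroy it with a spark emitter, while projectiles, items and actors without the IDamagable interface are ignored.
; Other damagable actors also destroy it with sparks, but only those not tagged Friendly receive damage through the AffectHealthMessage call and trigger the hit sound.
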(event EventBeginPlay
  (bind _astwin_stick_mode (Utilities|Casting|CastToTwinStickMode (Game|GetGameMode)))
  (Default|LaserSound3 (Variables|/Game/Blueprints/TwinStickMode.TwinStickMode_C|GetAudioManagerReference _astwin_stick_mode)))

(event EventTick
  (params (DeltaSeconds :type Float%20%28single-precision%29)))

(event Collision|EventActorBeginOverlap
  (params (OtherActor :type Actor%20Object%20Reference))
  (bind _returnvalue (Transformation|GetActorTransform))
  (if (Actor|ActorHasTag OtherActor "Wall")
    (CallFunction|DestroywithSparks)
    (elif (not (Actor|ActorHasTag OtherActor "Projectile"))
      (if (Utilities|DoesObjectImplementInterface OtherActor "/Game/Blueprints/iDamagable.iDamagable_C")
        (if (not (Actor|ActorHasTag OtherActor "Item"))
          (if (not (Actor|ActorHasTag OtherActor "Friendly"))
            (Class|IDamagable|AffectHealth(Message) OtherActor (Variables|Default|GetDamage))
            (bind _astwin_stick_mode (Utilities|Casting|CastToTwinStickMode (Game|GetGameMode)))
            (Default|BulletHitSound (Variables|/Game/Blueprints/TwinStickMode.TwinStickMode_C|GetAudioManagerReference _astwin_stick_mode)))
          (Effects|SpawnEmitteratLocation "/Game/StarterContent/Particles/LaserSparks.LaserSparks" (.location _returnvalue) (.rotation _returnvalue) (.scale _returnvalue) true "AutoRelease")
          (Actor|DestroyActor))))))

(fn ConstructionScript)

(fn DestroywithSparks
  (bind _returnvalue (Transformation|GetActorTransform))
  (Effects|SpawnEmitteratLocation "/Game/StarterContent/Particles/LaserSparks.LaserSparks" (.location _returnvalue) (.rotation _returnvalue) (.scale _returnvalue) true "AutoRelease")
  (Actor|DestroyActor))