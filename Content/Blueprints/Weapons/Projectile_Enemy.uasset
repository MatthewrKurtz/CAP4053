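; Enemy laser projectile for a twin-stick game that damages friendly actors on overlap.
; On spawn it plays a laser sound through the game mode's audio manager.
; On overlap it ignores enemies, projectiles, items and anything not implementing IDamagable.
; Other hits spawn pooled sparks and destroy the projectile, with damage sent by interface message only to Friendly-tagged actors.
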(event EventBeginPlay
  (bind _astwin_stick_mode (Utilities|Casting|CastToTwinStickMode (Game|GetGameMode)))
  (Default|LaserSound3 (Variables|/Game/Blueprints/TwinStickMode.TwinStickMode_C|GetAudioManagerReference _astwin_stick_mode)))

(event Collision|EventActorBeginOverlap
  (params (OtherActor :type Actor%20Object%20Reference))
  (bind _returnvalue (Transformation|GetActorTransform))
  (if (not (Actor|ActorHasTag OtherActor "Enemy"))
    (if (not (Actor|ActorHasTag OtherActor "Projectile"))
      (if (Utilities|DoesObjectImplementInterface OtherActor "/Game/Blueprints/iDamagable.iDamagable_C")
        (if (not (Actor|ActorHasTag OtherActor "Item"))
          (if (Actor|ActorHasTag OtherActor "Friendly")
            (Class|IDamagable|AffectHealth(Message) OtherActor (Variables|Default|GetDamage)))
          (Effects|SpawnEmitteratLocation "/Game/StarterContent/Particles/LaserSparks.LaserSparks" (.location _returnvalue) (.rotation _returnvalue) (.scale _returnvalue) true "AutoRelease")
          (Actor|DestroyActor))))))

(fn ConstructionScript
  (|CallParentFunction))