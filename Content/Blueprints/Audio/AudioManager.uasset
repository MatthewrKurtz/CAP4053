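; Central audio manager that exposes one function per game sound for combat, monsters, footsteps, UI, pickups and atmosphere.
; BeginPlay fills attack, growl and death cue arrays, which are played randomly at the player pawn's location, and starts the ambient track.
; Footsteps repeat on a toggled looping timer; most other sounds play in 2D.
; Tick polls the hero's room layout and, on a match, stops ambience and plays boss atmosphere every frame, without a guard.
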(event EventBeginPlay
  (Variables|Default|SetattackSounds (Utilities|Array|MakeArray "/Game/Blueprints/Audio/assets/punch_Cue.punch_Cue" "/Game/Blueprints/Audio/assets/knife_swing_Cue.knife_swing_Cue" "/Game/Blueprints/Audio/assets/creature/hit/attack/Monster-7_Cue.Monster-7_Cue" "/Game/Blueprints/Audio/assets/creature/hit/attack/Monster-8_Cue.Monster-8_Cue"))
  (Variables|Default|SetgrowlSounds (Utilities|Array|MakeArray "/Game/Blueprints/Audio/assets/creature/growl/Monster-1_Cue.Monster-1_Cue" "/Game/Blueprints/Audio/assets/creature/growl/Monster-2_Cue.Monster-2_Cue" "/Game/Blueprints/Audio/assets/creature/growl/Monster-3_Cue.Monster-3_Cue" "/Game/Blueprints/Audio/assets/creature/growl/Monster-4_Cue.Monster-4_Cue" "/Game/Blueprints/Audio/assets/creature/growl/Monster-5_Cue.Monster-5_Cue" "/Game/Blueprints/Audio/assets/creature/growl/Monster-6_Cue.Monster-6_Cue"))
  (Variables|Default|SetdeathSounds (Utilities|Array|MakeArray "/Game/Blueprints/Audio/assets/creature/hit/death/monster-9_Cue.monster-9_Cue" "/Game/Blueprints/Audio/assets/creature/hit/death/monster-10_Cue.monster-10_Cue" "/Game/Blueprints/Audio/assets/creature/hit/death/monster-11_Cue.monster-11_Cue" "/Game/Blueprints/Audio/assets/creature/hit/death/monster-12_Cue.monster-12_Cue" "/Game/Blueprints/Audio/assets/creature/hit/death/monster-13_Cue.monster-13_Cue" "/Game/Blueprints/Audio/assets/creature/hit/death/monster-14_Cue.monster-14_Cue" "/Game/Blueprints/Audio/assets/creature/hit/death/monster-15_Cue.monster-15_Cue" "/Game/Blueprints/Audio/assets/creature/hit/death/monster-16_Cue.monster-16_Cue" "/Game/Blueprints/Audio/assets/creature/hit/death/monster-17_Cue.monster-17_Cue" "/Game/Blueprints/Audio/assets/creature/hit/death/monster-18_Cue.monster-18_Cue"))
  (bind _sound (CallFunction|AtmosphereSound)))

(event EventTick
  (params (DeltaSeconds :type Float%20%28single-precision%29))
  (bind _ashero_character (Utilities|Casting|CastToHeroCharacter (Game|Player|GetPlayerPawn 0)))
  (if (Utilities|Enum|Equal(Enum) (.RoomLayout (Utilities|Struct|BreakFRoomInfo (Variables|/Game/Blueprints/Rooms/Room.Room_C|GetRoomInfo (Variables|/Game/Blueprints/HeroCharacter.HeroCharacter_C|GetCurrentRoom _ashero_character)))) "NewEnumerator8")
    (Audio|Components|Audio|Stop (stale EventBeginPlay _sound))
    (CallFunction|BossAtmosphereSound)))

(fn Footstep
  (params (Toggle :type Boolean))
  (bind _self self)
  (if Toggle
    (Utilities|Time|SetTimerbyFunctionName _self "FootstepSound" 0.5 true)
    (else
      (Utilities|Time|ClearTimerbyFunctionName _self "FootstepSound"))))

(fn FootstepSound
  (Audio|SpawnSound2D "/Game/Blueprints/Audio/assets/footstep1_Cue.footstep1_Cue" 1.0 1.0 0.0 0))

(fn AtmosphereSound
  (bind _returnvalue (Audio|SpawnSound2D "/Game/Blueprints/Audio/assets/atmosphere/Atmosphere_Cue.Atmosphere_Cue" 1.0 1.0 0.0 0))
  (return _returnvalue))

(fn AttackSound
  (bind _attacksounds (Variables|Default|GetattackSounds))
  (Audio|SpawnSoundatLocation (Utilities|Array|Get(acopy) _attacksounds (Math|Random|RandomInteger (Utilities|Array|Length _attacksounds))) (Transformation|GetActorLocation (Game|Player|GetPlayerPawn 0)) "0, 0, 0" 1.0 1.0 0.0 0 0))

(fn GrowlSound
  (bind _growlsounds (Variables|Default|GetgrowlSounds))
  (Audio|SpawnSoundatLocation (Utilities|Array|Get(acopy) _growlsounds (Math|Random|RandomInteger (Utilities|Array|Length _growlsounds))) (Transformation|GetActorLocation (Game|Player|GetPlayerPawn 0)) "0, 0, 0" 1.0 1.0 0.0 0 0))

(fn DeathSound
  (bind _deathsounds (Variables|Default|GetdeathSounds))
  (Audio|SpawnSoundatLocation (Utilities|Array|Get(acopy) _deathsounds (Math|Random|RandomInteger (Utilities|Array|Length _deathsounds))) (Transformation|GetActorLocation (Game|Player|GetPlayerPawn 0)) "0, 0, 0" 1.0 1.0 0.0 0 0))

(fn BigAttackSound
  (Audio|PlaySound2D "/Game/Blueprints/Audio/assets/creature/big/Creature_Monster_Attack_09_Cue.Creature_Monster_Attack_09_Cue" 1.0 1.0 0.0 0 0))

(fn BigDeathSound
  (Audio|PlaySound2D "/Game/Blueprints/Audio/assets/creature/big/Creature_Alien_Death_01_Cue.Creature_Alien_Death_01_Cue" 1.0 1.0 0.0 0 0))

(fn BigGrowlSound
  (Audio|PlaySound2D "/Game/Blueprints/Audio/assets/creature/big/Creature_Monster_Pain_01_Cue.Creature_Monster_Pain_01_Cue" 1.0 1.0 0.0 0 0))

(fn LaserSound1
  (Audio|PlaySoundatLocation "/Game/Blueprints/Audio/assets/weapons/laser1_Cue.laser1_Cue" (Transformation|GetActorLocation (Game|Player|GetPlayerPawn 0)) "0, 0, 0" 1.0 1.0 0.0 0 0 0))

(fn LaserSound2
  (Audio|PlaySoundatLocation "/Game/Blueprints/Audio/assets/weapons/laser4_Cue.laser4_Cue" (Transformation|GetActorLocation (Game|Player|GetPlayerPawn 0)) "0, 0, 0" 1.0 1.0 0.0 0 0 0))

(fn LaserSound3
  (Audio|PlaySoundatLocation "/Game/Blueprints/Audio/assets/weapons/laser5_Cue.laser5_Cue" (Transformation|GetActorLocation (Game|Player|GetPlayerPawn 0)) "0, 0, 0" 1.0 1.0 0.0 0 0 0))

(fn LaserSound4
  (Audio|PlaySoundatLocation "/Game/Blueprints/Audio/assets/weapons/laser6_Cue.laser6_Cue" (Transformation|GetActorLocation (Game|Player|GetPlayerPawn 0)) "0, 0, 0" 1.0 1.0 0.0 0 0 0))

(fn LaserSound5
  (Audio|PlaySoundatLocation "/Game/Blueprints/Audio/assets/weapons/laser8_Cue.laser8_Cue" (Transformation|GetActorLocation (Game|Player|GetPlayerPawn 0)) "0, 0, 0" 1.0 1.0 0.0 0 0 0))

(fn BulletHitSound
  (Audio|PlaySound2D "/Game/Blueprints/Audio/assets/weapons/bullet_hit_Cue.bullet_hit_Cue" 1.0 1.0 0.0 0 0))

(fn BulletFlybySound
  (Audio|PlaySound2D "/Game/Blueprints/Audio/assets/weapons/bullet_flyby_Cue.bullet_flyby_Cue" 1.0 1.0 0.0 0 0))

(fn ExplosionSound
  (Audio|PlaySound2D "/Game/StarterContent/Audio/Explosion_Cue.Explosion_Cue" 1.0 1.0 0.0 0 0))

(fn BossAtmosphereSound
  (Audio|PlaySound2D "/Game/Blueprints/Audio/assets/atmosphere/boss_atmosphere_Cue.boss_atmosphere_Cue" 1.0 1.0 0.0 0 0))

(fn TitleAtmosphereSound
  (Audio|PlaySound2D "/Game/Blueprints/Audio/assets/atmosphere/title_atmosphere_Cue.title_atmosphere_Cue" 1.0 1.0 0.0 0 0))

(fn RocketSound
  (Audio|PlaySound2D "/Game/Blueprints/Audio/assets/weapons/rocket_Cue.rocket_Cue" 1.0 1.0 0.0 0 0))

(fn UISound1
  (Audio|PlaySound2D "/Game/Blueprints/Audio/assets/UI/UI1_Cue.UI1_Cue" 1.0 1.0 0.0 0 0))

(fn UISound3
  (Audio|PlaySound2D "/Game/Blueprints/Audio/assets/UI/UI3_Cue.UI3_Cue" 1.0 1.0 0.0 0 0))

(fn UISound2
  (Audio|PlaySound2D "/Game/Blueprints/Audio/assets/UI/UI2_Cue.UI2_Cue" 1.0 1.0 0.0 0 0))

(fn HealthUpSound
  (Audio|PlaySound2D "/Game/Blueprints/Audio/assets/healthUp_Cue.healthUp_Cue" 1.0 1.0 0.0 0 0))

(fn DoorOpenSound
  (Audio|PlaySound2D "/Game/Blueprints/Audio/assets/DoorOpen_Cue.DoorOpen_Cue" 1.0 1.0 0.0 0 0))

(fn GunPickUpSound
  (Audio|PlaySound2D "/Game/Blueprints/Audio/assets/gunPickUp_Cue.gunPickUp_Cue" 1.0 1.0 0.0 0 0))

(fn TeleportSound
  (Audio|PlaySound2D "/Game/Blueprints/Audio/assets/creature/teleport_Cue.teleport_Cue" 1.0 1.0 0.0 0 0))

(fn GunPowerSound
  (bind _returnvalue (Audio|SpawnSound2D "/Game/Blueprints/Audio/assets/weapons/power_Cue.power_Cue" 1.0 1.0 0.0 0))
  (return _returnvalue))