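; Twin-stick shooter enemy character that ChangeEnemyType configures as one of seven types, setting mesh, animation, color and stats, then updating its AI controller.
; Hero overlap flags melee attackers as attacking or detonates Explosive ones, while timers repeat damage and projectile fire.
; Patrol and Teleport types pick random room-grid points.
; Death awards score, plays type-based audio, optionally explodes, leaves the room and may drop an item.
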(event Custom|Explode
  (bind _capsulecomponent (Variables|Default|GetCapsuleComponent))
  ;[1 1 1] Explode and Die
  (if (not (Variables|Default|GetisDead))
    (Collision|SetCollisionResponsetoChannel _capsulecomponent "ECC_WorldDynamic" "ECR_Ignore")
    (Collision|SetCollisionResponsetoChannel _capsulecomponent "ECC_Pawn" "ECR_Ignore")
    (Class|Pawn|DetachfromControllerPendingDestroy)
    (Game|SpawnActorfromClass "/Game/Blueprints/Enemies/Explosion.Explosion_C" (Transformation|GetActorTransform) "Undefined" 0 0)
    (Actor|DestroyActor)
    (bind _astwin_stick_mode (Utilities|Casting|CastToTwinStickMode (Game|GetGameMode)))
    (Default|ExplosionSound (Variables|/Game/Blueprints/TwinStickMode.TwinStickMode_C|GetAudioManagerReference _astwin_stick_mode))))

(event Custom|DamageTheHero
  ;[1 1 1] Damage
  (Default|AffectHealth (Variables|Default|GetHero) (Variables|Default|GetDamage))
  (Utilities|Time|SetTimerbyFunctionName 0 "DamageTheHero" (/ 1.0 (Variables|Default|GetAttacksPerSecond)) true)
  (bind _astwin_stick_mode (Utilities|Casting|CastToTwinStickMode (Game|GetGameMode)))
  (if (Math|Boolean|ORBoolean (Utilities|Enum|Equal(Enum) "NewEnumerator0" (Variables|Default|GetEnemyType)) (Utilities|Enum|Equal(Enum) "NewEnumerator4" (Variables|Default|GetEnemyType)) (Utilities|Enum|Equal(Enum) "NewEnumerator2" (Variables|Default|GetEnemyType)))
    (Default|BigAttackSound (Variables|/Game/Blueprints/TwinStickMode.TwinStickMode_C|GetAudioManagerReference _astwin_stick_mode))
    (else
      (Default|AttackSound (Variables|/Game/Blueprints/TwinStickMode.TwinStickMode_C|GetAudioManagerReference _astwin_stick_mode)))))

(event Custom|RotateToPlayer
  ;[1 1 1] Rotate (with Speed)
  (Transformation|SetActorRotation (Math|Interpolation|RInterpTo (Math|Rotator|FindLookatRotation (Transformation|GetActorLocation) (Transformation|GetActorLocation (Game|GetPlayerCharacter 0))) "0, 0, 0" (Utilities|Time|GetWorldDeltaSeconds) (Variables|Default|GetInterpolationSpeed))))

(event Custom|Fly
  ;[1 1 1] Fly
  (if (Variables|Default|GetFlying)
    _))

(event Custom|ShootProjectile
  ;[1 1 1] Shoot Projectile
  (if (Variables|Default|GetProjectile)
    (Game|SpawnActorfromClass "/Game/Blueprints/Weapons/Projectile_Enemy.Projectile_Enemy_C" (Transformation|GetWorldTransform (Variables|Default|GetEnemyProjectileSpawn)) "Undefined" 0 0)))

(event Custom|ShootAndRotate
  ;[1 1 1] Shoot and Rotate
  (if (not (Variables|Default|GetisDead))
    (Utilities|FlowControl|Sequence
      (:then_0
        (CallFunction|RotatetoPlayer))
      (:then_1
        (Utilities|FlowControl|DoOnce false
          (:Completed
            (Utilities|Time|SetTimerbyFunctionName 0 "ShootProjectile" (/ 1.0 (Variables|Default|GetProjectiles%20Per%20Second)) true)))))
    (else
      (Utilities|Time|ClearTimerbyFunctionName 0 "ShootProjectile"))))

(event Custom|ChangeEnemyType
  (params (EnemyType :type EnemyType%20Enum :default "NewEnumerator0"))
  (bind _output_get (Variables|Default|SetEnemyType EnemyType))
  (Development|PrintString (Utilities|String|EnumtoString _output_get))
  (Variables|Default|SetSpawnLocation (Transformation|GetActorLocation self))
  (Utilities|FlowControl|Sequence
    (:then_0
      (switch Utilities|FlowControl|Switch|SwitchonEnemyType (Variables|Default|GetEnemyType)
        (:NewEnumerator0
          (Variables|Default|SetEnemyColor (Variables|Default|GetBlue))
          ;[1 1 1] BeginPlay
          (Variables|/Script/Engine.CharacterMovementComponent|SetMaxWalkSpeed (Variables|Character|GetCharacterMovement) (Variables|Default|GetSpeed))
          (Class|SkinnedMeshComponent|SetSkeletalMesh (Variables|Character|GetMesh) "/Game/anim/charger/idle/Charger_Mesh.Charger_Mesh" true)
          (Components|SkeletalMesh|SetAnimInstanceClass (Variables|Character|GetMesh) "/Game/anim/charger/idle/ChargerAnimBlueprint.ChargerAnimBlueprint_C"))
        (:NewEnumerator1
          (Variables|Default|SetEnemyColor (Variables|Default|GetTurquoise))
          (Class|SkinnedMeshComponent|SetSkeletalMesh (Variables|Character|GetMesh) "/Game/anim/patrol/idle/PatrolMesh.PatrolMesh" true)
          (Components|SkeletalMesh|SetAnimInstanceClass (Variables|Character|GetMesh) "/Game/anim/patrol/idle/PatrolAnimBlueprint.PatrolAnimBlueprint_C")
          (CallFunction|CreatePoints :!label _label)
          (Variables|/Script/Engine.CharacterMovementComponent|SetMaxWalkSpeed (Variables|Character|GetCharacterMovement) (Variables|Default|GetSpeed)))
        (:NewEnumerator3
          (Variables|Default|SetEnemyColor (Variables|Default|GetPink))
          (Class|SkinnedMeshComponent|SetSkeletalMesh (Variables|Character|GetMesh) "/Game/anim/swarm/idle/SwarmMesh.SwarmMesh" true)
          (Components|SkeletalMesh|SetAnimInstanceClass (Variables|Character|GetMesh) "/Game/anim/swarm/idle/SwarmAnimBlueprint.SwarmAnimBlueprint_C")
          (Transformation|SetWorldScale3D (Variables|Character|GetMesh) "0.500000,0.500000,0.500000")
          (Variables|/Script/Engine.CharacterMovementComponent|SetMaxWalkSpeed (Variables|Character|GetCharacterMovement) (* (Variables|Default|GetSpeed) 2.0))
          (Variables|Default|SetDamage (/ (Variables|Default|GetDamage) 3.0))
          (Variables|Default|SetHealth (/ (Variables|Default|GetHealth) 3.0)))
        (:NewEnumerator2
          (Variables|Default|SetEnemyColor (Variables|Default|GetYellow))
          (Variables|/Script/Engine.CharacterMovementComponent|SetMaxWalkSpeed (Variables|Character|GetCharacterMovement) (* (Variables|Default|GetSpeed) 2.0))
          (Class|SkinnedMeshComponent|SetSkeletalMesh (Variables|Character|GetMesh) "/Game/anim/explosive/idle/ExplosiveMesh.ExplosiveMesh" true)
          (Components|SkeletalMesh|SetAnimInstanceClass (Variables|Character|GetMesh) "/Game/anim/explosive/idle/ExplosiveAnimBlueprint.ExplosiveAnimBlueprint_C"))
        (:NewEnumerator4
          (Variables|Default|SetEnemyColor (Variables|Default|GetGreen))
          (Class|SkinnedMeshComponent|SetSkeletalMesh (Variables|Character|GetMesh) "/Game/anim/fasthorz/idle/FastHorzMesh.FastHorzMesh" true)
          (Components|SkeletalMesh|SetAnimInstanceClass (Variables|Character|GetMesh) "/Game/anim/fasthorz/idle/FastHorzAnimBlueprint.FastHorzAnimBlueprint_C")
          (Variables|/Script/Engine.CharacterMovementComponent|SetMaxWalkSpeed (Variables|Character|GetCharacterMovement) (Variables|Default|GetSpeed))
          (Variables|/Script/Engine.CharacterMovementComponent|SetMaxAcceleration (Variables|Character|GetCharacterMovement) 5e+04))
        (:NewEnumerator5
          (Variables|Default|SetEnemyColor (Variables|Default|GetRed))
          (Class|SkinnedMeshComponent|SetSkeletalMesh (Variables|Character|GetMesh) "/Game/anim/teleport/attack/TeleportMesh.TeleportMesh" true)
          (Components|SkeletalMesh|SetAnimInstanceClass (Variables|Character|GetMesh) "/Game/anim/teleport/attack/TeleportAnimBlueprint.TeleportAnimBlueprint_C")
          (goto _label))
        (:NewEnumerator6
          (Class|SkinnedMeshComponent|SetSkeletalMesh (Variables|Character|GetMesh) "/Game/anim/turret/attack/TurretMesh.TurretMesh" true)
          (Components|SkeletalMesh|SetAnimInstanceClass (Variables|Character|GetMesh) "/Game/anim/turret/attack/TurretAnimBlueprint.TurretAnimBlueprint_C"))))
    (:then_1
      (CallFunction|ChangeBaseColor)
      (bind _asai_character_controller (Utilities|Casting|CastToAi_CharacterController (Pawn|GetController)))
      (Default|UpdateAi _asai_character_controller))))

(event Custom|ShootAndRotate_Moving
  ;[1 1 1] Shoot and Rotate Behavior with isMoving
  (if (not (Variables|Default|GetisDead))
    (Utilities|FlowControl|Sequence
      (:then_0
        (if (Math|Float|NearlyEqual(Float) (Math|Vector|VectorLength (Transformation|GetVelocity)) 0.0 1e-06)
          (Variables|Default|SetisMoving false)
          (Variables|Default|SetisAttacking true)
          (else
            (Variables|Default|SetisMoving true)
            (Variables|Default|SetisAttacking false))))
      (:then_1
        (if (not (Variables|Default|GetisMoving))
          (Utilities|FlowControl|Sequence
            (:then_0
              (CallFunction|RotatetoPlayer))
            (:then_1
              (Utilities|FlowControl|DoOnce false :!label _label
                (:Completed
                  (Utilities|Time|SetTimerbyFunctionName 0 "ShootProjectile" (/ 1.0 (Variables|Default|GetProjectiles%20Per%20Second)) true)))))
          (else
            (Utilities|Time|ClearTimerbyFunctionName 0 "ShootProjectile")
            (goto _label Reset)))))
    (else
      (Utilities|Time|ClearTimerbyFunctionName 0 "ShootProjectile"))))

(event Custom|StopFiring
  (Utilities|Time|ClearTimerbyFunctionName 0 "ShootProjectile"))

(event Custom|Fire
  (Utilities|Time|SetTimerbyFunctionName 0 "ShootProjectile" (/ 1.0 (Variables|Default|GetProjectiles%20Per%20Second)) true))

(event Custom|CreatePoints
  ;[1 1 1] Create Points
  (bind _location (Default|GetGridTileLocation (Variables|Default|GetcurrentRoom) (Math|Random|RandomInteger 9) (Math|Random|RandomInteger 9)))
  (bind _location_2 (Default|GetGridTileLocation (Variables|Default|GetcurrentRoom) (Math|Random|RandomInteger 9) (Math|Random|RandomInteger 9)))
  (bind _location_3 (Default|GetGridTileLocation (Variables|Default|GetcurrentRoom) (Math|Random|RandomInteger 9) (Math|Random|RandomInteger 9)))
  (bind _location_4 (Default|GetGridTileLocation (Variables|Default|GetcurrentRoom) (Math|Random|RandomInteger 9) (Math|Random|RandomInteger 9)))
  (Variables|Default|SetPoints (Utilities|Array|MakeArray _location _location_2 _location_3 _location_4))
  (CallFunction|GetRandomPoint))

(event EventTick
  (params (DeltaSeconds :type Float%20%28single-precision%29))
  ;[1 1 1] Event Tick
)

(event Collision|EventActorBeginOverlap
  (params (OtherActor :type Actor%20Object%20Reference))
  ;[1 1 1] Actor Begin Overlap
  (bind _ashero_character (Utilities|Casting|CastToHeroCharacter OtherActor)
    (:then
      (Variables|Default|SetHero _ashero_character)
      (switch Utilities|FlowControl|Switch|SwitchonEnemyType (Variables|Default|GetEnemyType)
        (:NewEnumerator0
          (Variables|Default|SetisAttacking true :!label _label))
        (:NewEnumerator3
          (goto _label))
        (:NewEnumerator2
          (CallFunction|Explode))
        (:NewEnumerator4
          (Variables|Default|SetAttacksPerSecond 2e+01)
          (goto _label))))
    (:CastFailed
      (Utilities|Casting|CastToDoor OtherActor))))

(event EventAffectHealth
  (params (Delta :type Float%20%28single-precision%29))
  (bind _capsulecomponent (Variables|Default|GetCapsuleComponent))
  ;[1 1 1] Death
  (Class|BaseCharacter|CalculateHealth Delta)
  (if (Variables|Default|GetisDead)
    (bind _astwin_stick_mode (Utilities|Casting|CastToTwinStickMode (Game|GetGameMode)))
    (if (Math|Boolean|ORBoolean (Utilities|Enum|Equal(Enum) "NewEnumerator0" (Variables|Default|GetEnemyType)) (Utilities|Enum|Equal(Enum) "NewEnumerator4" (Variables|Default|GetEnemyType)) (Utilities|Enum|Equal(Enum) "NewEnumerator2" (Variables|Default|GetEnemyType)))
      (Default|BigDeathSound (Variables|/Game/Blueprints/TwinStickMode.TwinStickMode_C|GetAudioManagerReference _astwin_stick_mode))
      (else
        (Default|DeathSound (Variables|/Game/Blueprints/TwinStickMode.TwinStickMode_C|GetAudioManagerReference _astwin_stick_mode))))
    (Default|IncrementScore _astwin_stick_mode (Variables|Default|GetScore))
    (Collision|SetCollisionResponsetoChannel _capsulecomponent "ECC_WorldDynamic" "ECR_Ignore")
    (Collision|SetCollisionResponsetoChannel _capsulecomponent "ECC_Pawn" "ECR_Ignore")
    (Class|Pawn|DetachfromControllerPendingDestroy)
    (Utilities|FlowControl|Delay 3.0)
    (if (Variables|Default|GetExplodeOnDeath)
      (Game|SpawnActorfromClass "/Game/Blueprints/Enemies/Explosion.Explosion_C" (Transformation|GetActorTransform) "Undefined" 0 0))
    (Default|RemoveEnemy (Variables|Default|GetcurrentRoom) self)
    (Utilities|FlowControl|Sequence
      (:then_0
        (if (<= (Math|Random|RandomFloat) (* (Variables|Default|GetPercentageChanceToDropItem) 0.01))
          (bind _returnvalue (Game|SpawnActorfromClass "/Game/Blueprints/Interactables/BP_BaseItem.BP_BaseItem_C" (Math|Transform|MakeTransform (Transformation|GetActorLocation self) "0, 0, 0" "1,1,1") "Undefined" 0 0))
          (Default|ChangeItemType _returnvalue "NewEnumerator6")))
      (:then_1
        (Actor|DestroyActor)))))

(event Collision|EventActorEndOverlap
  (params (OtherActor :type Actor%20Object%20Reference))
  (if (== OtherActor (Variables|Default|GetHero))
    (switch Utilities|FlowControl|Switch|SwitchonEnemyType (Variables|Default|GetEnemyType)
      (:NewEnumerator0
        (Utilities|Time|ClearTimerbyFunctionName 0 "DamageTheHero" :!label _label)
        (Utilities|FlowControl|Delay 1.0)
        (Variables|Default|SetisAttacking false))
      (:NewEnumerator3
        (goto _label))
      (:NewEnumerator4
        (Utilities|Time|ClearTimerbyFunctionName 0 "DamageTheHero")
        (Variables|Default|SetisAttacking false)))))

(event EventBeginPlay)

(fn ConstructionScript)

(fn GetRandomPoint
  (Variables|Default|SetCurrent%20Destination (Math|Random|RandomInteger (Utilities|Array|Length (Variables|Default|GetPoints)))))

(fn ChangeBaseColor
  (bind _returnvalue (Rendering|Material|CreateDynamicMaterialInstance (Variables|Character|GetMesh) 0 0 "None" :!class /Script/Engine.PrimitiveComponent))
  (bind _output_get (Variables|Default|SetDyna%20Mat _returnvalue))
  (Rendering|Material|SetVectorParameterValue _output_get "BodyColor" (Variables|Default|GetEnemyColor) :!class /Script/Engine.MaterialInstanceDynamic))

(fn GetNextPatrolPoint
  (bind _output_get (Variables|Default|SetNextPatrolPoint (Utilities|Array|Get(acopy) (Variables|Default|GetPoints) (Variables|Default|GetCurrent%20Destination))))
  (bind _output_get_2 (Variables|Default|SetCurrent%20Destination (+ (Variables|Default|GetCurrent%20Destination) 1)))
  (if (>= _output_get_2 (Utilities|Array|Length (Variables|Default|GetPoints)))
    (Variables|Default|SetCurrent%20Destination 0))
  (return _output_get))

(fn SetPatrolPointsfromRoom
  (params (XY-PatrolCoordinates :type Array%20of%20Vectors))
  (for _array_element XY-PatrolCoordinates
    (bind _location (Default|GetGridTileLocation (Variables|Default|GetcurrentRoom) (Math|Float|Truncate (.x _array_element)) (Math|Float|Truncate (.y _array_element))))
    (Utilities|Array|Add (Variables|Default|GetPoints) _location)))