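; AI controller that drives EnemyCharacter pawns, choosing a movement behavior from EnemyType shortly after BeginPlay.
; Charger, Swarm and Explosive repeatedly chase the player, while Patrol and Teleport periodically move or jump to the pawn's current point, then pick another randomly.
; Fast Horz loops between slow X steps and fast Y dashes, steered by hard-coded world-coordinate bounds.
; All AI moves go straight to their goal without pathfinding.
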(event Custom|TrackPlayer
  ;[1 1 1] Track Player
  (AI|Navigation|MovetoActor (Game|GetPlayerCharacter 0) -1.0 true false true 0))

(event Custom|TeleportToPoint
  ;[1 1 1] TeleportToPoint
  (Utilities|FlowControl|Sequence
    (:then_0
      (bind _asenemy_character (Utilities|Casting|CastToEnemyCharacter (Pawn|GetControlledPawn)))
      (Transformation|SetActorLocation _asenemy_character (Utilities|Array|Get(acopy) (Variables|/Game/Blueprints/Enemies/EnemyCharacter.EnemyCharacter_C|GetPoints _asenemy_character) (Variables|/Game/Blueprints/Enemies/EnemyCharacter.EnemyCharacter_C|GetCurrent%20Destination _asenemy_character)) false false))
    (:then_1
      (Default|GetRandomPoint _asenemy_character))))

(event Custom|FastHorz
  ;[1 1 1] Fast Horizontal Movement
  (bind _asenemy_character (Utilities|Casting|CastToEnemyCharacter (Pawn|GetControlledPawn)))
  (if (> (.Y (Math|Vector|BreakVector (Transformation|GetActorLocation _asenemy_character))) -1.9255e+05)
    (Variables|/Script/Engine.CharacterMovementComponent|SetMaxWalkSpeed (Variables|/Script/Engine.Character|GetCharacterMovement _asenemy_character) 2.5e+03 :!label _label)
    (AI|Navigation|MovetoLocation (Math|Vector|MakeVector (.X (Math|Vector|BreakVector (Transformation|GetActorLocation _asenemy_character))) (- (.Y (Math|Vector|BreakVector (Transformation|GetActorLocation _asenemy_character))) 1.5e+03) (.Z (Math|Vector|BreakVector (Transformation|GetActorLocation _asenemy_character)))) -1.0 true false false true 0)
    (Utilities|FlowControl|Delay 1.3)
    (CallFunction|SlowVert)
    (elif (< (.Y (Math|Vector|BreakVector (Transformation|GetActorLocation _asenemy_character))) -1.9385e+05)
      (Variables|/Script/Engine.CharacterMovementComponent|SetMaxWalkSpeed (Variables|/Script/Engine.Character|GetCharacterMovement _asenemy_character) 2.5e+03)
      (AI|Navigation|MovetoLocation (Math|Vector|MakeVector (.X (Math|Vector|BreakVector (Transformation|GetActorLocation _asenemy_character))) (+ (.Y (Math|Vector|BreakVector (Transformation|GetActorLocation _asenemy_character))) 1.5e+03) (.Z (Math|Vector|BreakVector (Transformation|GetActorLocation _asenemy_character)))) -1.0 true false false true 0)
      (Utilities|FlowControl|Delay 1.3)
      (CallFunction|SlowVert)
      (else
        (goto _label)))))

(event Custom|SlowVert
  ;[1 1 1] Slow Vertical Movement
  (bind _asenemy_character (Utilities|Casting|CastToEnemyCharacter (Pawn|GetControlledPawn)))
  (Variables|/Script/Engine.CharacterMovementComponent|SetMaxWalkSpeed (Variables|/Script/Engine.Character|GetCharacterMovement _asenemy_character) 2e+02)
  (if (< (.X (Math|Vector|BreakVector (Transformation|GetActorLocation _asenemy_character))) 6.8063e+05)
    (Variables|Default|SetGoingUp true)
    (elif (> (.X (Math|Vector|BreakVector (Transformation|GetActorLocation _asenemy_character))) 6.8215e+05)
      (Variables|Default|SetGoingUp false)))
  (if (Variables|Default|GetGoingUp)
    (AI|Navigation|MovetoLocation (Math|Vector|MakeVector (+ (.X (Math|Vector|BreakVector (Transformation|GetActorLocation _asenemy_character))) 2e+02) (.Y (Math|Vector|BreakVector (Transformation|GetActorLocation _asenemy_character))) (.Z (Math|Vector|BreakVector (Transformation|GetActorLocation _asenemy_character)))) -1.0 true false false true 0)
    (Utilities|FlowControl|Delay 1.0)
    (CallFunction|FastHorz)
    (else
      (AI|Navigation|MovetoLocation (Math|Vector|MakeVector (- (.X (Math|Vector|BreakVector (Transformation|GetActorLocation _asenemy_character))) 2e+02) (.Y (Math|Vector|BreakVector (Transformation|GetActorLocation _asenemy_character))) (.Z (Math|Vector|BreakVector (Transformation|GetActorLocation _asenemy_character)))) -1.0 true false false true 0)
      (Utilities|FlowControl|Delay 0.5)
      (CallFunction|FastHorz))))

(event Custom|MoveToPoint
  ;[1 1 1] MoveToPoint
  (Utilities|FlowControl|Sequence
    (:then_0
      (bind _asenemy_character (Utilities|Casting|CastToEnemyCharacter (Pawn|GetControlledPawn)))
      (AI|Navigation|MovetoLocation (Utilities|Array|Get(acopy) (Variables|/Game/Blueprints/Enemies/EnemyCharacter.EnemyCharacter_C|GetPoints _asenemy_character) (Variables|/Game/Blueprints/Enemies/EnemyCharacter.EnemyCharacter_C|GetCurrent%20Destination _asenemy_character)) -1.0 true false false true 0))
    (:then_1
      (Default|GetRandomPoint _asenemy_character))))

(event EventBeginPlay
  ;[1 1 1] Begin Play
  (Utilities|FlowControl|Delay 0.1)
  (bind _asenemy_character (Utilities|Casting|CastToEnemyCharacter (Pawn|GetControlledPawn)))
  (switch Utilities|FlowControl|Switch|SwitchonEnemyType (Variables|/Game/Blueprints/Enemies/EnemyCharacter.EnemyCharacter_C|GetEnemyType _asenemy_character)
    (:NewEnumerator0
      (Utilities|Time|SetTimerbyFunctionName 0 "TrackPlayer" 0.5 true :!label _label))
    (:NewEnumerator1
      (Utilities|Time|SetTimerbyFunctionName 0 "MoveToPoint" 5.0 true))
    (:NewEnumerator3
      (goto _label))
    (:NewEnumerator2
      (goto _label))
    (:NewEnumerator4
      (Utilities|Time|SetTimerbyFunctionName 0 "SlowVert" 0.1))
    (:NewEnumerator5
      (Utilities|Time|SetTimerbyFunctionName 0 "TeleportToPoint" 5.0 true))))

(fn ConstructionScript)