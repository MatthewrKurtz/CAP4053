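; Enemy spawner Blueprint that places AI-controlled EnemyCharacter pawns inside a spawn volume, up to a maximum count.
; Each SpawnEnemy call picks a random point within the SpawnVolume box and uses SpawnAIFromClass to spawn one enemy there.
; It passes its CurrentRoom to the new enemy and increments the spawn counter, which is never decremented here, so the limit covers total spawns.
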(event Custom|SpawnEnemy
  (bind _spawnvolume (Variables|Default|GetSpawnVolume))
  (if (< (Variables|Default|GetNumberOfEnemiesSpawned) (Variables|Default|GetMaxEnemies))
    (if true
      (bind _returnvalue (AI|SpawnAIFromClass "/Game/Blueprints/Enemies/EnemyCharacter.EnemyCharacter_C" 0 (Math|Random|RandomPointinBoundingBox (Transformation|GetWorldLocation _spawnvolume) (Components|Box|GetScaledBoxExtent _spawnvolume)) "0, 0, 0" false))
      (bind _asenemy_character (Utilities|Casting|CastToEnemyCharacter _returnvalue))
      (Variables|/Game/Blueprints/Enemies/EnemyCharacter.EnemyCharacter_C|SetcurrentRoom _asenemy_character (Variables|Default|GetcurrentRoom))
      (Math|Integer|IncrementInt (Variables|Default|GetNumberOfEnemiesSpawned)))))

(fn ConstructionScript)