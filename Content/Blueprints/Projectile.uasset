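; Projectile actor that deals damage to what it hits through the IDamagable interface.
; On overlap it ignores other projectiles, items and actors without that interface, and sends its Damage through AffectHealthMessage unless the target is tagged Friendly.
; Friendly and damaged targets alike trigger a LaserSparks emitter at the projectile's transform and destroy it.
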(event EventBeginPlay)

(event EventTick
  (params (DeltaSeconds :type Float%20%28single-precision%29)))

(event Collision|EventActorBeginOverlap
  (params (OtherActor :type Actor%20Object%20Reference))
  (bind _returnvalue (Transformation|GetActorTransform))
  (if (not (Actor|ActorHasTag OtherActor "Projectile"))
    (if (Utilities|DoesObjectImplementInterface OtherActor "/Game/Blueprints/iDamagable.iDamagable_C")
      (if (not (Actor|ActorHasTag OtherActor "Item"))
        (if (not (Actor|ActorHasTag OtherActor "Friendly"))
          (Class|IDamagable|AffectHealth(Message) OtherActor (Variables|Default|GetDamage)))
        (Effects|SpawnEmitteratLocation "/Game/StarterContent/Particles/LaserSparks.LaserSparks" (.location _returnvalue) (.rotation _returnvalue) (.scale _returnvalue) true "AutoRelease")
        (Actor|DestroyActor)))))

(fn ConstructionScript)