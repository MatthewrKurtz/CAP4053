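; Base weapon Blueprint that fires projectiles automatically while the trigger is held.
; PullTrigger fires at once through a DoOnce and starts a looping timer set by RoundsPerSecond.
; ReleaseTrigger clears that timer and resets the DoOnce, so re-pulling fires immediately with no cooldown.
; Fire spawns the WeaponInfo projectile type at ProjectileSpawnPoint, with ChangeWeaponSpread randomizing only yaw within the weapon's spread.
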(event Custom|PullTrigger
  ;[1 1 1] Fire in Rounds Per Second When Trigger is Pulled/Released
  (Utilities|FlowControl|DoOnce false
    (:Completed
      (CallFunction|Fire)
      (Utilities|Time|SetTimerbyFunctionName 0 "Fire" (/ 1.0 (Variables|Default|GetRoundsPerSecond)) true))))

(event Custom|ReleaseTrigger
  ;[1 1 1] Fire in Rounds Per Second When Trigger is Pulled/Released
  (Utilities|Time|ClearTimerbyFunctionName 0 "Fire")
  (Utilities|FlowControl|DoOnce false) ; enters at Reset
)

(event Custom|Fire
  (bind _weaponinfo (Variables|Default|GetWeaponInfo))
  (bind (_spread _projectiletype) (Utilities|Struct|BreakFWeaponInfo _weaponinfo))
  ;[1 1 1] Fire (Spawn Projectile)
  (switch Utilities|FlowControl|Switch|SwitchonEProjectileType _projectiletype
    (:NewEnumerator0
      (Variables|Default|SetProjectileType "/Game/Blueprints/Projectile.Projectile_C")
      (Game|SpawnActorfromClass (Variables|Default|GetProjectileType) (CallFunction|ChangeWeaponSpread _spread) "Undefined" 0 0))))

(fn ConstructionScript)

(fn ChangeWeaponSpread
  (params (Spread%20Amount :type Float%20%28single-precision%29))
  (bind _projectilespawnpoint (Variables|Default|GetProjectileSpawnPoint))
  (bind _returnvalue (Transformation|GetWorldTransform _projectilespawnpoint))
  (return (Math|Transform|MakeTransform (.location _returnvalue) (Math|Rotator|MakeRotator (.roll (.rotation _returnvalue)) (.pitch (.rotation _returnvalue)) (+ (.yaw (.rotation _returnvalue)) (Math|Random|RandomFloatinRange Spread%20Amount (* Spread%20Amount -1.0)))) (.scale _returnvalue))))