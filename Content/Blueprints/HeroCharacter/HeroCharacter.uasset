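; Player hero character for a twin-stick shooter, handling movement, stick-driven aim and fire, weapons, inventory and death respawn through TwinStickMode.
; Each tick highlights a registered interactable by dot product with gun forward, and also adds a new weapon-inventory widget.
; Pickups, item use and primary/secondary inputs replace the weapon actor attached to GunTemp.
; Weapon dropping is unwired; equipment functions are stubs.
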(event EventBeginPlay
  (bind _guntemp (Variables|Default|GetGunTemp))
  (Utilities|FlowControl|Sequence
    (:then_0
      (bind _returnvalue (Game|SpawnActorfromClass "/Game/Blueprints/Weapons/BaseWeapon.BaseWeapon_C" (Transformation|GetWorldTransform _guntemp) "Undefined" 0 0))
      (bind _output_get (Variables|Default|SetWeapon%28nonInteractable%29 _returnvalue))
      ;[1 1 1] SetupWeapon
      (Transformation|AttachComponentToComponent _output_get _guntemp "" "SnapToTarget" "KeepWorld" "KeepWorld" true))
    (:then_1
      ;[1 1 1] Adjust to Game Mode
      (bind _astwin_stick_mode (Utilities|Casting|CastToTwinStickMode (Game|GetGameMode)))
      (bind _output_get_2 (Variables|Default|SetGameMode _astwin_stick_mode))
      (Variables|/Game/Blueprints/TwinStickMode.TwinStickMode_C|SetPlayerSpawnTransform _output_get_2 (Transformation|GetActorTransform)))
    (:then_2
      ;[1 1 1] Setup HUD
      (bind _returnvalue_2 (UserInterface|CreateWidget "/Game/Blueprints/UI/TwinStickHUD.TwinStickHUD_C"))
      (UserInterface|Viewport|AddtoViewport _returnvalue_2 0))))

(event EventUseItem
  (params (itemInfo :type F%20Item%20Info%20Structure))
  ;[1 1 1] Use Item
  (switch Utilities|FlowControl|Switch|SwitchonEItemType (.itemtype itemInfo)
    (:NewEnumerator1
      (bind _asbase_weapon (Utilities|Casting|CastToBaseWeaponClass (.itemclass itemInfo)))
      (CallFunction|ChangeWeapon(notInteractable) _asbase_weapon))))

(event EventTick
  (params (DeltaSeconds :type Float%20%28single-precision%29))
  ;[1 1 1] Interaction Handling
  (CallFunction|UpdateBestInteractable)
  (bind _returnvalue (UserInterface|CreateWidget "/Game/Blueprints/UI/UI_WeaponInventory.UI_WeaponInventory_C"))
  (UserInterface|Viewport|AddtoViewport _returnvalue 0)
  (Development|PrintString (Utilities|String|EnumtoString (.WeaponType (Utilities|Struct|BreakFWeaponInfo (Variables|/Game/Blueprints/Weapons/BaseWeapon.BaseWeapon_C|GetWeaponInfo (Variables|Default|GetWeapon%28nonInteractable%29)))))))

(event EventAffectHealth
  (params (Delta :type Float%20%28single-precision%29))
  ;[1 1 1] Health
  (Class|BaseCharacter|CalculateHealth Delta)
  (if (Variables|Default|GetisDead)
    (Input|DisableInput (Game|GetPlayerController 0))
    (Utilities|FlowControl|Delay 3.0)
    (Default|RespawnPlayer (Variables|Default|GetGameMode))
    (Actor|DestroyActor self)))

(event EventRegisterInteractable
  (params (Interactable :type BP%20Base%20Interactable%20Object%20Reference))
  ;[1 1 1] Interaction Handling
  (CallFunction|HandleRegisterInteractable Interactable))

(event EventUnregisterInteractable
  (params (Interactable :type BP%20Base%20Interactable%20Object%20Reference))
  ;[1 1 1] Interaction Handling
  (CallFunction|HandleUnregisterInteractable Interactable))

(event EventPickup
  (params (ItemInfo :type F%20Item%20Info%20Structure))
  (bind (_itemtype _itemname _itemimage _itemclass) (Utilities|Struct|BreakFItemInfo ItemInfo))
  (bind _inventoryreference (Variables|Default|GetInventoryReference))
  (switch Utilities|FlowControl|Switch|SwitchonEItemType _itemtype
    (:NewEnumerator1
      (CallFunction|ChangeWeapon(notInteractable) _itemclass)
      (Utilities|Array|Add (Variables|Default|GetInventory) ItemInfo)
      (Utilities|IsValid _inventoryreference
        (:Is%20Valid
          (Default|CreateInventory _inventoryreference))))))

(event EventUnuseItem
  (params (ItemInfo :type F%20Item%20Info%20Structure))
  ;[1 1 1] Unuse Item
  (CallFunction|UnattachEquipment))

(event Input|ActionEvents|InputActionInteract
  (params (Key :type Key%20Structure))
  (bind _highlightedinteractable (Variables|Default|GetHighlightedInteractable))
  ;[1 1 1] Interact (F)
  (:Pressed
    (Utilities|IsValid _highlightedinteractable
      (:Is%20Valid
        (Class|BPIInteract|Interaction(Message) _highlightedinteractable self)))))

(event Input|ActionEvents|InputActionInventory
  (params (Key :type Key%20Structure))
  (bind _returnvalue (Game|GetPlayerController 0))
  (bind _returnvalue_2 (Game|GetPlayerController 0))
  ;[1 1 1] Create The Inventory
  (:Pressed
    (if (Variables|Default|GetIsInventoryOpen)
      (Widget|RemovefromParent (Variables|Default|GetInventoryReference))
      (Input|SetInputModeGameOnly _returnvalue)
      (Variables|/Script/Engine.PlayerController|SetbShowMouseCursor _returnvalue false)
      (Variables|Default|SetIsInventoryOpen false)
      (else
        (bind _returnvalue_3 (UserInterface|CreateWidget "/Game/Blueprints/UI/UI_inventory.UI_inventory_C"))
        (bind _output_get (Variables|Default|SetInventoryReference _returnvalue_3))
        (UserInterface|Viewport|AddtoViewport _output_get 1)
        (Input|SetInputModeGameandUI _returnvalue_2 _output_get "DoNotLock" true)
        (Variables|/Script/Engine.PlayerController|SetbShowMouseCursor _returnvalue_2 true)
        (Variables|Default|SetIsInventoryOpen true)))))

(event Input|ActionEvents|InputActionSwitchToSecondary
  (params (Key :type Key%20Structure))
  ;[1 1 1] Switch To Secondary
  (:Pressed
    (CallFunction|ChangeWeapon(notInteractable) "/Game/Blueprints/Weapons/Weapon_Trident.Weapon_Trident_C")))

(event Input|ActionEvents|InputActionSwitchToPrimary
  (params (Key :type Key%20Structure))
  ;[1 1 1] Switch to Primary
  (:Pressed
    (CallFunction|ChangeWeapon(notInteractable) "/Game/Blueprints/Weapons/BaseWeapon.BaseWeapon_C")))

(event Input|AxisEvents|InputAxisMoveUp
  (params (AxisValue :type Float%20%28single-precision%29))
  ;[1 1 1] Movement
  (Pawn|Input|AddMovementInput "1.000000, 0, 0" AxisValue false))

(event Input|AxisEvents|InputAxisMoveRight
  (params (AxisValue :type Float%20%28single-precision%29))
  ;[1 1 1] Movement
  (Pawn|Input|AddMovementInput "0.000000,1.000000, 0" AxisValue false))

(event Input|AxisEvents|InputAxisLookUp
  (params (AxisValue :type Float%20%28single-precision%29))
  (bind _weapon_noninteractable_ (Variables|Default|GetWeapon%28nonInteractable%29))
  ;[1 1 1] Rotation
  (if (> (Math|Vector|VectorLength (Math|Vector|MakeVector AxisValue (stale Input|AxisEvents|InputAxisLookRight AxisValue) 0.0)) 0.25)
    (Pawn|SetControlRotation (Game|GetPlayerController 0) (Math|Conversions|RotationFromXVector (Math|Vector|MakeVector AxisValue (stale Input|AxisEvents|InputAxisLookRight AxisValue) 0.0)))
    (Default|PullTrigger _weapon_noninteractable_)
    (else
      (Default|ReleaseTrigger _weapon_noninteractable_))))

(event Input|AxisEvents|InputAxisLookRight
  (params (AxisValue :type Float%20%28single-precision%29))
  (bind _weapon_noninteractable_ (Variables|Default|GetWeapon%28nonInteractable%29))
  ;[1 1 1] Rotation
  (if (> (Math|Vector|VectorLength (Math|Vector|MakeVector (stale Input|AxisEvents|InputAxisLookUp AxisValue) AxisValue 0.0)) 0.25)
    (Pawn|SetControlRotation (Game|GetPlayerController 0) (Math|Conversions|RotationFromXVector (Math|Vector|MakeVector (stale Input|AxisEvents|InputAxisLookUp AxisValue) AxisValue 0.0)))
    (Default|PullTrigger _weapon_noninteractable_)
    (else
      (Default|ReleaseTrigger _weapon_noninteractable_))))

(fn ConstructionScript)

(fn HandleRegisterInteractable
  (params (Interactable :type BP%20Base%20Interactable%20Object%20Reference))
  (Utilities|Array|AddUnique (Variables|Default|GetInteractables) Interactable))

(fn HandleUnregisterInteractable
  (params (Interactable :type BP%20Base%20Interactable%20Object%20Reference))
  (Utilities|Array|RemoveItem (Variables|Default|GetInteractables) Interactable))

(fn UpdateBestInteractable
  (if (> (Utilities|Array|Length (Variables|Default|GetInteractables)) 0)
    (CallFunction|GetBestInteractable)
    (else
      (CallFunction|SetBestInteractable))))

(fn GetBestInteractable
  (bind _guntemp (Variables|Default|GetGunTemp))
  (LocalVariables|SetInteractableVariables (Utilities|Struct|MakeFInteractableVariables -1.0 0))
  (for _array_element (Variables|Default|GetInteractables)
    (if (and (> (Math|Vector|DotProduct (Math|Vector|Normalize (- (Physics|GetCenterOfMass (Variables|/Game/Blueprints/Interactables/BP_BaseInteractable.BP_BaseInteractable_C|GetInteractableMesh _array_element) "None") (Transformation|GetWorldLocation _guntemp))) (Math|Vector|GetForwardVector _guntemp)) (LocalVariables|GetMaxDotProduct)) (>= (Math|Vector|DotProduct (Math|Vector|Normalize (- (Physics|GetCenterOfMass (Variables|/Game/Blueprints/Interactables/BP_BaseInteractable.BP_BaseInteractable_C|GetInteractableMesh _array_element) "None") (Transformation|GetWorldLocation _guntemp))) (Math|Vector|GetForwardVector _guntemp)) (.dot (LocalVariables|GetInteractableVariables))))
      (LocalVariables|SetInteractableVariables (Utilities|Struct|MakeFInteractableVariables (Math|Vector|DotProduct (Math|Vector|Normalize (- (Physics|GetCenterOfMass (Variables|/Game/Blueprints/Interactables/BP_BaseInteractable.BP_BaseInteractable_C|GetInteractableMesh _array_element) "None") (Transformation|GetWorldLocation _guntemp))) (Math|Vector|GetForwardVector _guntemp)) _array_element))
      (LocalVariables|SetMaxDotProduct (Math|Vector|DotProduct (Math|Vector|Normalize (- (Physics|GetCenterOfMass (Variables|/Game/Blueprints/Interactables/BP_BaseInteractable.BP_BaseInteractable_C|GetInteractableMesh _array_element) "None") (Transformation|GetWorldLocation _guntemp))) (Math|Vector|GetForwardVector _guntemp)))))
  (Utilities|IsValid (.interactable (LocalVariables|GetInteractableVariables))
    (:Is%20Valid
      (CallFunction|SetBestInteractable (.interactable (LocalVariables|GetInteractableVariables))))
    (:Is%20Not%20Valid
      (CallFunction|SetBestInteractable))))

(fn SetBestInteractable
  (params (Interactable :type BP%20Base%20Interactable%20Object%20Reference))
  (Utilities|IsValid Interactable
    (:Is%20Valid
      (if (!= Interactable (Variables|Default|GetHighlightedInteractable))
        (bind _highlightedinteractable (Variables|Default|GetHighlightedInteractable)
          (:then
            (Default|SetHighlight _highlightedinteractable false))
          (:else
            _)))
      (bind _output_get (Variables|Default|SetHighlightedInteractable Interactable))
      (Default|SetHighlight _output_get true))
    (:Is%20Not%20Valid
      (bind _highlightedinteractable_2 (Variables|Default|GetHighlightedInteractable)
        (:then
          (Default|SetHighlight _highlightedinteractable_2 false)
          (Variables|Default|SetHighlightedInteractable 0))
        (:else)))))

(fn HasSpaceinInventory
  (return (< (Utilities|Array|Length (Variables|Default|GetInventory)) (Variables|Default|GetInventorySize))))

(fn AttachEquipment
  (params (ItemInfo :type F%20Item%20Info%20Structure))
  (switch Utilities|FlowControl|Switch|SwitchonESlotType (.ItemSlot (Utilities|Struct|BreakFItemInfo ItemInfo))))

(fn UnattachEquipment
  (params (ItemInfo :type F%20Item%20Info%20Structure)))

(fn ChangeWeapon
  (params (WeaponClass :type BP%20Base%20Gun%20Pickup%20Class%20Reference))
  (bind _guntemp (Variables|Default|GetGunTemp))
  (bind _returnvalue (Game|SpawnActorfromClass WeaponClass (Transformation|GetWorldTransform _guntemp) "Undefined" 0 0))
  (Utilities|IsValid (Variables|Default|GetWeapon)
    (:Is%20Valid
      (Actor|DestroyActor (Variables|Default|GetWeapon))
      (bind _output_get (Variables|Default|SetWeapon _returnvalue))
      (Transformation|AttachComponentToComponent _output_get _guntemp "None" "SnapToTarget" "KeepWorld" "KeepRelative" true))))

(fn ChangeWeapon(notInteractable)
  (params (WeaponClass :type Base%20Weapon%20Class%20Reference))
  (bind _guntemp (Variables|Default|GetGunTemp))
  (bind _returnvalue (Game|SpawnActorfromClass WeaponClass (Transformation|GetWorldTransform _guntemp) "Undefined" 0 0))
  (Utilities|IsValid (Variables|Default|GetWeapon%28nonInteractable%29)
    (:Is%20Valid
      (Actor|DestroyActor (Variables|Default|GetWeapon%28nonInteractable%29))
      (bind _output_get (Variables|Default|SetWeapon%28nonInteractable%29 _returnvalue))
      (Transformation|AttachComponentToComponent _output_get _guntemp "None" "SnapToTarget" "KeepWorld" "KeepRelative" true))))

(fn DropCurrentWeapon
  (switch Utilities|FlowControl|Switch|SwitchonEWeaponType (.weapontype (Variables|/Game/Blueprints/Weapons/BaseWeapon.BaseWeapon_C|GetWeaponInfo (Variables|Default|GetWeapon%28nonInteractable%29)))
    (:NewEnumerator0
      (CallFunction|SpawnClass "/Game/Blueprints/Interactables/Weapons/BP_BaseGunPickup.BP_BaseGunPickup_C"))
    (:NewEnumerator1
      (CallFunction|SpawnClass "/Game/Blueprints/Interactables/Weapons/BP_TridentShotPickup.BP_TridentShotPickup_C"))
    (:NewEnumerator2
      (CallFunction|SpawnClass "/Game/Blueprints/Interactables/Weapons/BP_HomingMissilePickup.BP_HomingMissilePickup_C"))
    (:NewEnumerator3
      (CallFunction|SpawnClass "/Game/Blueprints/Interactables/Weapons/BP_ShotgunPickup.BP_ShotgunPickup_C"))
    (:NewEnumerator4
      (CallFunction|SpawnClass "/Game/Blueprints/Interactables/Weapons/BP_ChargeShotPickup.BP_ChargeShotPickup_C"))))

(fn SpawnClass
  (params (ClassToSpawn :type BP%20Base%20Item%20Class%20Reference))
  (Game|SpawnActorfromClass ClassToSpawn (Transformation|GetWorldTransform (Variables|Character|GetMesh)) "Undefined" 0 0))